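; Character component that builds a modular, gendered body from skin-set data assets, with switchable PBR or cel-shaded sets.
; On BeginPlay it polls for the owner's face mesh, then attaches copy-pose skeletal meshes per body slot and async-loads the initial skin.
; Equipping picks the male or female mesh and creates dynamic materials.
; Color, scalar and texture overrides, filtered by material name, are cached and reapplied after part or gender changes.
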(event Custom|Load%20Skin
  (params (Asset :type Object%20Soft%20Object%20Reference))
  (bind _object (Utilities|AsyncLoadAsset Asset)
    (:Completed
      (bind _asbp_data_skin_sets (Utilities|Casting|CastToBP_Data_SkinSets _object))
      (Equipping|SetPartsfromDataAsset _asbp_data_skin_sets))))

(event EventBeginPlay
  (Utilities|Time|SetTimerbyFunctionName 0 "Set Initial References" 0.3 true))

(fn SelectPartbyEnum
  (params (Enum :type E_ModularParts%20Enum :default "NewEnumerator0"))
  (bind _keys (Utilities|Map|Keys (Variables|References|GetParts%20Array)))
  (for _array_element _keys
    (if (Utilities|Enum|Equal(Enum) (.Part (Utilities|Struct|BreakF_ModularPart (.Value (Utilities|Map|Find (Variables|References|GetParts%20Array) _array_element)))) Enum)
      (return _array_element))))

(fn AddMeshComponents
  (Utilities|FlowControl|Sequence
    (:then_1
      ;[1 1 1] Hair
      (bind _returnvalue (Game|AddComponentbyClass (Variables|References|GetCharacter) "/Script/Engine.SkeletalMeshComponent" false))
      (bind _output_get (Variables|Default|SetHair _returnvalue))
      (Transformation|AttachComponentToComponent _output_get (Variables|Default|GetFace) "None" "SnapToTarget" "SnapToTarget" "SnapToTarget" true)
      (Rendering|SetVisibility _output_get false false)
      (Class|SkeletalMeshComponent|SetAnimClass _output_get "/Game/Polyart/SharedResources/Characters/AnimationStuff/AnimationBlueprints/ABP_CopyPose.ABP_CopyPose_C")
      (Utilities|Map|Add (Variables|References|GetParts%20Array) (Variables|Default|GetHair) (Utilities|Struct|MakeF_ModularPart 0 0 "NewEnumerator0" 0 0 "(GameplayTags=)" "(GameplayTags=)")))
    (:then_2
      ;[1 1 1] Torso
      (bind _returnvalue_2 (Game|AddComponentbyClass (Variables|References|GetCharacter) "/Script/Engine.SkeletalMeshComponent" false))
      (bind _output_get_2 (Variables|Default|SetTorso _returnvalue_2))
      (Transformation|AttachComponentToComponent _output_get_2 (Variables|Default|GetFace) "None" "SnapToTarget" "SnapToTarget" "SnapToTarget" true)
      (Rendering|SetVisibility _output_get_2 false false)
      (Class|SkeletalMeshComponent|SetAnimClass _output_get_2 "/Game/Polyart/SharedResources/Characters/AnimationStuff/AnimationBlueprints/ABP_CopyPose.ABP_CopyPose_C")
      (Utilities|Map|Add (Variables|References|GetParts%20Array) (Variables|Default|GetTorso) (Utilities|Struct|MakeF_ModularPart 0 0 "NewEnumerator2" 0 0 "(GameplayTags=)" "(GameplayTags=)")))
    (:then_3
      ;[1 1 1] Shoulders
      (bind _returnvalue_3 (Game|AddComponentbyClass (Variables|References|GetCharacter) "/Script/Engine.SkeletalMeshComponent" false))
      (bind _output_get_3 (Variables|Default|SetShoulders _returnvalue_3))
      (Transformation|AttachComponentToComponent _output_get_3 (Variables|Default|GetFace) "None" "SnapToTarget" "SnapToTarget" "SnapToTarget" true)
      (Rendering|SetVisibility _output_get_3 false false)
      (Class|SkeletalMeshComponent|SetAnimClass _output_get_3 "/Game/Polyart/SharedResources/Characters/AnimationStuff/AnimationBlueprints/ABP_CopyPose.ABP_CopyPose_C")
      (Utilities|Map|Add (Variables|References|GetParts%20Array) (Variables|Default|GetShoulders) (Utilities|Struct|MakeF_ModularPart 0 0 "NewEnumerator3" 0 0 "(GameplayTags=)" "(GameplayTags=)")))
    (:then_4
      ;[1 1 1] Legs
      (bind _returnvalue_4 (Game|AddComponentbyClass (Variables|References|GetCharacter) "/Script/Engine.SkeletalMeshComponent" false))
      (bind _output_get_4 (Variables|Default|SetLegs _returnvalue_4))
      (Transformation|AttachComponentToComponent _output_get_4 (Variables|Default|GetFace) "None" "SnapToTarget" "SnapToTarget" "SnapToTarget" true)
      (Rendering|SetVisibility _output_get_4 false false)
      (Class|SkeletalMeshComponent|SetAnimClass _output_get_4 "/Game/Polyart/SharedResources/Characters/AnimationStuff/AnimationBlueprints/ABP_CopyPose.ABP_CopyPose_C")
      (Utilities|Map|Add (Variables|References|GetParts%20Array) (Variables|Default|GetLegs) (Utilities|Struct|MakeF_ModularPart 0 0 "NewEnumerator6" 0 0 "(GameplayTags=)" "(GameplayTags=)")))
    (:then_5
      ;[1 1 1] Shoes
      (bind _returnvalue_5 (Game|AddComponentbyClass (Variables|References|GetCharacter) "/Script/Engine.SkeletalMeshComponent" false))
      (bind _output_get_5 (Variables|Default|SetShoes _returnvalue_5))
      (Transformation|AttachComponentToComponent _output_get_5 (Variables|Default|GetFace) "None" "SnapToTarget" "SnapToTarget" "SnapToTarget" true)
      (Rendering|SetVisibility _output_get_5 false false)
      (Class|SkeletalMeshComponent|SetAnimClass _output_get_5 "/Game/Polyart/SharedResources/Characters/AnimationStuff/AnimationBlueprints/ABP_CopyPose.ABP_CopyPose_C")
      (Utilities|Map|Add (Variables|References|GetParts%20Array) (Variables|Default|GetShoes) (Utilities|Struct|MakeF_ModularPart 0 0 "NewEnumerator7" 0 0 "(GameplayTags=)" "(GameplayTags=)")))
    (:then_6
      ;[1 1 1] Gloves
      (bind _returnvalue_6 (Game|AddComponentbyClass (Variables|References|GetCharacter) "/Script/Engine.SkeletalMeshComponent" false))
      (bind _output_get_6 (Variables|Default|SetGloves _returnvalue_6))
      (Transformation|AttachComponentToComponent _output_get_6 (Variables|Default|GetFace) "None" "SnapToTarget" "SnapToTarget" "SnapToTarget" true)
      (Rendering|SetVisibility _output_get_6 false false)
      (Class|SkeletalMeshComponent|SetAnimClass _output_get_6 "/Game/Polyart/SharedResources/Characters/AnimationStuff/AnimationBlueprints/ABP_CopyPose.ABP_CopyPose_C")
      (Utilities|Map|Add (Variables|References|GetParts%20Array) (Variables|Default|GetGloves) (Utilities|Struct|MakeF_ModularPart 0 0 "NewEnumerator4" 0 0 "(GameplayTags=)" "(GameplayTags=)")))
    (:then_7
      ;[1 1 1] Hips
      (bind _returnvalue_7 (Game|AddComponentbyClass (Variables|References|GetCharacter) "/Script/Engine.SkeletalMeshComponent" false))
      (bind _output_get_7 (Variables|Default|SetHips _returnvalue_7))
      (Transformation|AttachComponentToComponent _output_get_7 (Variables|Default|GetFace) "None" "SnapToTarget" "SnapToTarget" "SnapToTarget" true)
      (Rendering|SetVisibility _output_get_7 false false)
      (Class|SkeletalMeshComponent|SetAnimClass _output_get_7 "/Game/Polyart/SharedResources/Characters/AnimationStuff/AnimationBlueprints/ABP_CopyPose.ABP_CopyPose_C")
      (Utilities|Map|Add (Variables|References|GetParts%20Array) (Variables|Default|GetHips) (Utilities|Struct|MakeF_ModularPart 0 0 "NewEnumerator5" 0 0 "(GameplayTags=)" "(GameplayTags=)")))
    (:then_8
      ;[1 1 1] Helmet
      (bind _returnvalue_8 (Game|AddComponentbyClass (Variables|References|GetCharacter) "/Script/Engine.SkeletalMeshComponent" false))
      (bind _output_get_8 (Variables|Default|SetHelmet _returnvalue_8))
      (Transformation|AttachComponentToComponent _returnvalue_8 (Variables|Default|GetFace) "None" "SnapToTarget" "SnapToTarget" "SnapToTarget" true)
      (Rendering|SetVisibility _output_get_8 false false)
      (Class|SkeletalMeshComponent|SetAnimClass _output_get_8 "/Game/Polyart/SharedResources/Characters/AnimationStuff/AnimationBlueprints/ABP_CopyPose.ABP_CopyPose_C")
      (Utilities|Map|Add (Variables|References|GetParts%20Array) (Variables|Default|GetHelmet) (Utilities|Struct|MakeF_ModularPart 0 0 "NewEnumerator8" 0 0 "(GameplayTags=)" "(GameplayTags=)")))))

(fn EquipPart
  (params (Part :type F%20Modular%20Part%20Structure) (Optional%20Material%20Name :type String) (Optional%20SKM%20Comp :type Skeletal%20Mesh%20Component%20Object%20Reference) (Optional%20Attatch%20Socket :type String))
  (bind (_malemesh _femalemesh _part) (Utilities|Struct|BreakF_ModularPart Part))
  (bind (_malemesh_2 _femalemesh_2 _part_2 _maleicon _femaleicon _tagstoadd _tagstoremove) (Utilities|Struct|BreakF_ModularPart Part))
  (LocalVariables|SetMesh (select (Variables|States|GetIs%20Male?) _malemesh _femalemesh))
  (LocalVariables|SetPartEnum _part)
  (Utilities|IsValid Optional%20SKM%20Comp
    (:Is%20Valid
      (bind _output_get (LocalVariables|SetComponent Optional%20SKM%20Comp))
      (Class|SkeletalMeshComponent|SetAnimClass _output_get "/Game/Polyart/SharedResources/Characters/AnimationStuff/AnimationBlueprints/ABP_CopyPose.ABP_CopyPose_C")
      (Transformation|AttachComponentToComponent _output_get (Variables|Default|GetFace) (select (Utilities|Array|IsEmpty Optional%20Attatch%20Socket) "None" (Utilities|String|StringToName Optional%20Attatch%20Socket)) "SnapToTarget" "SnapToTarget" "KeepRelative" true))
    (:Is%20Not%20Valid
      (LocalVariables|SetComponent (Getters|SelectPartbyEnum (LocalVariables|GetPartEnum)))))
  (Utilities|Map|Add (Variables|References|GetParts%20Array) (LocalVariables|GetComponent) Part)
  (Utilities|FlowControl|Sequence
    (:then_0
      ;[1 1 1] Change Meshes and Materials
      (bind _mesh (LocalVariables|GetMesh)
        (:then
          (Components|SkeletalMesh|SetSkeletalMeshAsset (LocalVariables|GetComponent) _mesh)
          (Rendering|SetVisibility (LocalVariables|GetComponent) true false)
          (for (_array_element _array_index) (Variables|/Script/Engine.SkeletalMesh|GetMaterials (LocalVariables|GetMesh))
            (bind _returnvalue (Rendering|Material|CreateDynamicMaterialInstance (.materialinterface _array_element) (select (Utilities|Array|IsEmpty Optional%20Material%20Name) (.materialslotname _array_element) (Utilities|String|StringToName Optional%20Material%20Name)) "None" :!class /Script/Engine.KismetMaterialLibrary))
            (Utilities|Array|Add (LocalVariables|GetTempMaterials) _returnvalue)
            (Rendering|Material|SetMaterial (LocalVariables|GetComponent) _array_index _returnvalue))
          (Utilities|Map|Add (Variables|References|GetDynamic%20Material%20Array) (LocalVariables|GetComponent) (Utilities|Struct|MakeF_DynMatArray (LocalVariables|GetTempMaterials)))
          (StateChanges|UpdateMaterialParameters))
        (:else
          (Rendering|SetVisibility (LocalVariables|GetComponent) false false))))
    (:then_1
      ;[1 1 1] Optional Tagging system for gameplay purposes (currently not used)
      (GameplayTags|AppendGameplayTagContainers (Variables|GameplayLogic|GetTag%20Container) _tagstoadd)
      (for _array_element_2 (GameplayTags|BreakGameplayTagContainer _tagstoremove)
        (GameplayTags|RemoveGameplayTag (Variables|GameplayLogic|GetTag%20Container) _array_element_2 :!class /Script/GameplayTags.BlueprintGameplayTagLibrary)))))

(fn SetPartsfromDataAsset
  (params (Data%20Asset :type BP%20Data%20Skin%20Sets%20Object%20Reference))
  (for _array_element (Variables|/Game/Polyart/SharedResources/Characters/DataAssets/BP_Data_SkinSets.BP_Data_SkinSets_C|GetParts Data%20Asset)
    (Equipping|EquipPart _array_element))
  (Components|Animation|SetAnimationMode (Variables|Default|GetFace) "AnimationBlueprint")
  (StateChanges|UpdateMaterialParameters))

(fn SetInitialReferences
  (bind _initial_parts (Variables|References|GetInitial%20Parts))
  (Variables|References|SetCharacter (Components|GetOwner))
  (bind _character (Variables|References|GetCharacter)
    (:then
      (bind _output_get (Variables|Default|SetFace (Actor|GetComponentbyClass _character "/Script/Engine.SkeletalMeshComponent")))
      (Utilities|IsValid _output_get
        (:Is%20Valid
          (Utilities|Time|ClearTimerbyFunctionName 0 "Set Initial References")
          (Utilities|Map|Add (Variables|References|GetParts%20Array) (Variables|Default|GetFace) (Utilities|Struct|MakeF_ModularPart 0 0 "NewEnumerator1" 0 0 "(GameplayTags=)" "(GameplayTags=)"))
          (Utilities|SetAnimInstancebyGender)
          (Initialize|AddMeshComponents)
          (CallFunction|LoadSkin (select (Variables|States|GetUse%20PBR?) (.pbr _initial_parts) (.celshaded _initial_parts))))))
    (:else)))

(fn ChangeGender
  (Variables|States|SetIs%20Male? (not (Variables|States|GetIs%20Male?)))
  (Utilities|SetAnimInstancebyGender)
  (bind _values (Utilities|Map|Values (Variables|References|GetParts%20Array)))
  (for _array_element _values
    (Equipping|EquipPart _array_element))
  (Components|Animation|SetAnimationMode (Variables|Default|GetFace) "AnimationBlueprint")
  (StateChanges|UpdateMaterialParameters)
  (Default|CallGenderChanged))

(fn ChangeShading(ShowcasePurposes)
  (bind _initial_parts (Variables|References|GetInitial%20Parts))
  (Variables|States|SetUse%20PBR? (not (Variables|States|GetUse%20PBR?)))
  (CallFunction|LoadSkin (select (Variables|States|GetUse%20PBR?) (.pbr _initial_parts) (.celshaded _initial_parts))))

(fn ChangeColors
  (params (Linear%20Color%20Params :type Array%20of%20F%20Name%20and%20Color%20Structures) (Float%20Params :type Array%20of%20F%20Name%20and%20Float%20Structures) (Texture%20Params :type Array%20of%20F%20Name%20and%20Texture%20Structures) (Optional%20Filter%20Tag :type String))
  (bind _values (Utilities|Map|Values (Variables|References|GetDynamic%20Material%20Array)))
  (for _array_element _values
    (for _array_element_2 (Utilities|Struct|BreakF_DynMatArray _array_element)
      (Utilities|IsValid _array_element_2
        (:Is%20Valid
          (bind _output_get (LocalVariables|SetCurrMat _array_element_2))
          (if (or (Utilities|String|Contains (Utilities|GetDisplayName _output_get) Optional%20Filter%20Tag) (Utilities|Array|IsEmpty Optional%20Filter%20Tag))
            (Utilities|FlowControl|Sequence
              (:then_0
                (for _array_element_3 Linear%20Color%20Params
                  (Rendering|Material|SetVectorParameterValue (LocalVariables|GetCurrMat) (.ParameterName (Utilities|Struct|BreakF_NameAndColor _array_element_3)) (.Color (Utilities|Struct|BreakF_NameAndColor _array_element_3)) :!class /Script/Engine.MaterialInstanceDynamic)
                  (Utilities|Map|Add (Variables|MaterialParameters|GetColor%20Material%20Parameters) (.ParameterName (Utilities|Struct|BreakF_NameAndColor _array_element_3)) (Utilities|Struct|MakeF_ColorParamHolder _array_element_3 Optional%20Filter%20Tag))))
              (:then_1
                (for _array_element_4 Float%20Params
                  (Rendering|Material|SetScalarParameterValue (LocalVariables|GetCurrMat) (.Name (Utilities|Struct|BreakF_NameAndFloat _array_element_4)) (.Float (Utilities|Struct|BreakF_NameAndFloat _array_element_4)) :!class /Script/Engine.MaterialInstanceDynamic)
                  (Utilities|Map|Add (Variables|MaterialParameters|GetScalar%20Material%20Parameters) (.Name (Utilities|Struct|BreakF_NameAndFloat _array_element_4)) (Utilities|Struct|MakeF_FloatParamHolder _array_element_4 Optional%20Filter%20Tag))))
              (:then_2
                (for _array_element_5 Texture%20Params
                  (Rendering|Material|SetTextureParameterValue (LocalVariables|GetCurrMat) (.ParameterName (Utilities|Struct|BreakF_NameAndTexture _array_element_5)) (select (Utilities|IsValid (select (Variables|States|GetIs%20Male?) (.MaleTexture (Utilities|Struct|BreakF_NameAndTexture _array_element_5)) (.FemaleTexture (Utilities|Struct|BreakF_NameAndTexture _array_element_5)))) (select (Variables|States|GetIs%20Male?) (.MaleTexture (Utilities|Struct|BreakF_NameAndTexture _array_element_5)) (.FemaleTexture (Utilities|Struct|BreakF_NameAndTexture _array_element_5))) "/Game/Polyart/SharedResources/Characters/Textures/BothChar/T_Black.T_Black"))
                  (Utilities|Map|Add (Variables|MaterialParameters|GetTexture%20Material%20Parameters) (.ParameterName (Utilities|Struct|BreakF_NameAndTexture _array_element_5)) (Utilities|Struct|MakeF_TextureParamHolder _array_element_5 Optional%20Filter%20Tag)))))))))))

(fn ResetColors
  (bind (_colors _floats_) (|DefaultSkinParams))
  (Utilities|FlowControl|Sequence
    (:then_0
      (bind _keys (Utilities|Map|Keys (Variables|MaterialParameters|GetColor%20Material%20Parameters)))
      (for _array_element _keys
        (Utilities|Array|Add (LocalVariables|GetColorParams) (Utilities|Struct|MakeF_NameAndColor _array_element "(R=0.000000,G=1.000000,B=1.000000,A=0.000000)"))))
    (:then_1
      (StateChanges|ChangeColors (LocalVariables|GetColorParams) (Utilities|Array|MakeArray "") (Utilities|Array|MakeArray "") "main"))
    (:then_2
      (StateChanges|ChangeColors _colors _floats_ (Utilities|Array|MakeArray "") "skin"))))

(fn UpdateMaterialParameters
  (bind _values (Utilities|Map|Values (Variables|References|GetDynamic%20Material%20Array)))
  (for _array_element _values
    (for _array_element_2 (Utilities|Struct|BreakF_DynMatArray _array_element)
      (Utilities|IsValid _array_element_2
        (:Is%20Valid
          (LocalVariables|SetCurr%20Mat _array_element_2)
          (Utilities|FlowControl|Sequence
            (:then_0
              (bind _values_2 (Utilities|Map|Values (Variables|MaterialParameters|GetColor%20Material%20Parameters)))
              (for _array_element_3 _values_2
                (if (or (Utilities|String|Contains (Utilities|GetDisplayName (LocalVariables|GetCurr%20Mat)) (.FilterTag (Utilities|Struct|BreakF_ColorParamHolder _array_element_3))) (Utilities|Array|IsEmpty (.FilterTag (Utilities|Struct|BreakF_ColorParamHolder _array_element_3))))
                  (Rendering|Material|SetVectorParameterValue (LocalVariables|GetCurr%20Mat) (.ParameterName (Utilities|Struct|BreakF_NameAndColor (.ColorParam (Utilities|Struct|BreakF_ColorParamHolder _array_element_3)))) (.Color (Utilities|Struct|BreakF_NameAndColor (.ColorParam (Utilities|Struct|BreakF_ColorParamHolder _array_element_3)))) :!class /Script/Engine.MaterialInstanceDynamic))))
            (:then_1
              (bind _values_3 (Utilities|Map|Values (Variables|MaterialParameters|GetScalar%20Material%20Parameters)))
              (for _array_element_4 _values_3
                (if (or (Utilities|String|Contains (Utilities|GetDisplayName (LocalVariables|GetCurr%20Mat)) (.FilterTag (Utilities|Struct|BreakF_FloatParamHolder _array_element_4))) (Utilities|Array|IsEmpty (.FilterTag (Utilities|Struct|BreakF_FloatParamHolder _array_element_4))))
                  (Rendering|Material|SetScalarParameterValue (LocalVariables|GetCurr%20Mat) (.Name (Utilities|Struct|BreakF_NameAndFloat (.FloatParam (Utilities|Struct|BreakF_FloatParamHolder _array_element_4)))) (.Float (Utilities|Struct|BreakF_NameAndFloat (.FloatParam (Utilities|Struct|BreakF_FloatParamHolder _array_element_4)))) :!class /Script/Engine.MaterialInstanceDynamic))))
            (:then_2
              (bind _values_4 (Utilities|Map|Values (Variables|MaterialParameters|GetTexture%20Material%20Parameters)))
              (for _array_element_5 _values_4
                (if (or (Utilities|String|Contains (Utilities|GetDisplayName (LocalVariables|GetCurr%20Mat)) (.FilterTag (Utilities|Struct|BreakF_TextureParamHolder _array_element_5))) (Utilities|Array|IsEmpty (.FilterTag (Utilities|Struct|BreakF_TextureParamHolder _array_element_5))))
                  (Rendering|Material|SetTextureParameterValue (LocalVariables|GetCurr%20Mat) (.ParameterName (Utilities|Struct|BreakF_NameAndTexture (.TextureParam (Utilities|Struct|BreakF_TextureParamHolder _array_element_5)))) (select (Variables|States|GetIs%20Male?) (.MaleTexture (Utilities|Struct|BreakF_NameAndTexture (.TextureParam (Utilities|Struct|BreakF_TextureParamHolder _array_element_5)))) (.FemaleTexture (Utilities|Struct|BreakF_NameAndTexture (.TextureParam (Utilities|Struct|BreakF_TextureParamHolder _array_element_5)))))))))))))))