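; Enemy turn logic for turn-based grid combat: a monster closes on the nearest living party member and attacks.
; RunEnemyTurn picks the target by Chebyshev distance, greedily steps one free adjacent tile toward it, attacks without a range check, then notifies the combat manager.
; Attacks use ResolveAttack, or a d6 auto-hit branch for a conditioned target.
; Lethal damage downs the target; the victory check runs only after non-lethal hits.
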(event EventBeginPlay)

(event Collision|EventActorBeginOverlap
  (params (OtherActor :type Actor%20Object%20Reference)))

(event EventTick
  (params (DeltaSeconds :type Float%20%28single-precision%29)))

(fn ConstructionScript)

(fn FindNearestPartyMember
  (params (ActiveCombatant :type S%20Combatant%20Structure))
  (bind _gridposition (Utilities|Struct|BreakS_Combatant ActiveCombatant))
  (bind (_x _y) (Math|Vector2D|BreakVector2D _gridposition))
  (LocalVariables|SetBestDist 999)
  (for _array_element (Variables|/Game/Blueprints/Combat/BP_CombatManager.BP_CombatManager_C|GetCombatants (Variables|Default|GetCombatManagerRef))
    (if (not (.IsMonster (Utilities|Struct|BreakS_Combatant _array_element)))
      (if (not (<= (.CurrentHP (Utilities|Struct|BreakS_Combatant _array_element)) 0))
        (if (< (Math|Integer|Max(Integer) (Math|Integer|Absolute(Integer) (- (Math|Float|Truncate (.X (Math|Vector2D|BreakVector2D (.GridPosition (Utilities|Struct|BreakS_Combatant _array_element))))) (Math|Float|Truncate _x))) (Math|Integer|Absolute(Integer) (- (Math|Float|Truncate (.Y (Math|Vector2D|BreakVector2D (.GridPosition (Utilities|Struct|BreakS_Combatant _array_element))))) (Math|Float|Truncate _y)))) (LocalVariables|GetBestDist))
          (LocalVariables|SetBestDist (Math|Integer|Max(Integer) (Math|Integer|Absolute(Integer) (- (Math|Float|Truncate (.X (Math|Vector2D|BreakVector2D (.GridPosition (Utilities|Struct|BreakS_Combatant _array_element))))) (Math|Float|Truncate _x))) (Math|Integer|Absolute(Integer) (- (Math|Float|Truncate (.Y (Math|Vector2D|BreakVector2D (.GridPosition (Utilities|Struct|BreakS_Combatant _array_element))))) (Math|Float|Truncate _y)))))
          (LocalVariables|SetBestTarget _array_element)
          (LocalVariables|SetbLocalFound true)))))
  (return (LocalVariables|GetBestTarget) (LocalVariables|GetbLocalFound)))

(fn MoveOneStepToward
  (params (ActiveCombatant :type S%20Combatant%20Structure) (Target :type S%20Combatant%20Structure))
  (bind (_combatantid _combatantname _isplayercontrolled _sourcecharacter _sourcemonster _ismonster _gridposition) (Utilities|Struct|BreakS_Combatant ActiveCombatant))
  (LocalVariables|SetTargetCombatant Target)
  (LocalVariables|SetActiveCombatantID _combatantid)
  (LocalVariables|SetActiveCombatantGridPos _gridposition)
  (LocalVariables|SetActiveCombatantGridX (.X (Math|Vector2D|BreakVector2D (LocalVariables|GetActiveCombatantGridPos))))
  (LocalVariables|SetActiveCombatantGridY (.Y (Math|Vector2D|BreakVector2D (LocalVariables|GetActiveCombatantGridPos))))
  (for _array_element (Default|GetAdjacentTiles (Variables|/Game/Blueprints/Combat/BP_CombatManager.BP_CombatManager_C|GetCombatGridRef (Variables|Default|GetCombatManagerRef)) (Math|Float|Truncate (LocalVariables|GetActiveCombatantGridX)) (Math|Float|Truncate (LocalVariables|GetActiveCombatantGridY)))
    (if (Default|IsTraversable (Variables|/Game/Blueprints/Combat/BP_CombatManager.BP_CombatManager_C|GetCombatGridRef (Variables|Default|GetCombatManagerRef)) (Math|Float|Truncate (.X (Math|Vector2D|BreakVector2D _array_element))) (Math|Float|Truncate (.Y (Math|Vector2D|BreakVector2D _array_element))))
      (if (not (Default|IsOccupied (Variables|/Game/Blueprints/Combat/BP_CombatManager.BP_CombatManager_C|GetCombatGridRef (Variables|Default|GetCombatManagerRef)) (Math|Float|Truncate (.X (Math|Vector2D|BreakVector2D _array_element))) (Math|Float|Truncate (.Y (Math|Vector2D|BreakVector2D _array_element)))))
        (if (< (Math|Integer|Max(Integer) (Math|Integer|Absolute(Integer) (- (Math|Float|Truncate (.X (Math|Vector2D|BreakVector2D (.GridPosition (Utilities|Struct|BreakS_Combatant (LocalVariables|GetTargetCombatant)))))) (Math|Float|Truncate (.X (Math|Vector2D|BreakVector2D _array_element))))) (Math|Integer|Absolute(Integer) (- (Math|Float|Truncate (.Y (Math|Vector2D|BreakVector2D (.GridPosition (Utilities|Struct|BreakS_Combatant (LocalVariables|GetTargetCombatant)))))) (Math|Float|Truncate (.Y (Math|Vector2D|BreakVector2D _array_element)))))) (LocalVariables|GetBestDist))
          (LocalVariables|SetBestDist (Math|Integer|Max(Integer) (Math|Integer|Absolute(Integer) (- (Math|Float|Truncate (.X (Math|Vector2D|BreakVector2D (.GridPosition (Utilities|Struct|BreakS_Combatant (LocalVariables|GetTargetCombatant)))))) (Math|Float|Truncate (.X (Math|Vector2D|BreakVector2D _array_element))))) (Math|Integer|Absolute(Integer) (- (Math|Float|Truncate (.Y (Math|Vector2D|BreakVector2D (.GridPosition (Utilities|Struct|BreakS_Combatant (LocalVariables|GetTargetCombatant)))))) (Math|Float|Truncate (.Y (Math|Vector2D|BreakVector2D _array_element)))))))
          (LocalVariables|SetBestTile _array_element)))))
  (Default|ClearOccupant (Variables|/Game/Blueprints/Combat/BP_CombatManager.BP_CombatManager_C|GetCombatGridRef (Variables|Default|GetCombatManagerRef)) (Math|Float|Truncate (LocalVariables|GetActiveCombatantGridX)) (Math|Float|Truncate (LocalVariables|GetActiveCombatantGridY)))
  (Default|SetOccupant (Variables|/Game/Blueprints/Combat/BP_CombatManager.BP_CombatManager_C|GetCombatGridRef (Variables|Default|GetCombatManagerRef)) (Math|Float|Truncate (.X (Math|Vector2D|BreakVector2D (LocalVariables|GetBestTile)))) (Math|Float|Truncate (.Y (Math|Vector2D|BreakVector2D (LocalVariables|GetBestTile)))) (LocalVariables|GetActiveCombatantID))
  (Default|UpdateCombatantGridPosition (Variables|Default|GetCombatManagerRef) (LocalVariables|GetActiveCombatantID) (LocalVariables|GetBestTile))
  (Default|MoveMarkertoTile (Variables|Default|GetCombatManagerRef) (LocalVariables|GetActiveCombatantID) (LocalVariables|GetBestTile)))

(fn RunEnemyTurn
  (params (ActiveCombatant :type S%20Combatant%20Structure))
  (bind _combatmanagerref (Variables|Default|GetCombatManagerRef))
  (bind (_neareesttarget _bfound) (CallFunction|FindNearestPartyMember ActiveCombatant))
  (if _bfound
    (CallFunction|MoveOneStepToward ActiveCombatant _neareesttarget)
    (CallFunction|ExecuteEnemyAttack ActiveCombatant _neareesttarget)
    (Default|OnActionComplete _combatmanagerref)
    (else
      (Default|OnActionComplete _combatmanagerref))))

(fn ExecuteEnemyAttack
  (params (ActiveCombatant :type S%20Combatant%20Structure) (Target :type S%20Combatant%20Structure))
  (bind (_combatantid _combatantname _isplayercontrolled _sourcecharacter _sourcemonster _ismonster _gridposition _currenthp _maxhp _defenserating _strikenumber _initiative _actionsremaining _movementrange _attacksremaining _hasactedthisround _conditions _tilesmovedthisturn _characterid) (Utilities|Struct|BreakS_Combatant Target))
  (bind _bhascondition (Default|HasCondition (Variables|Default|GetCombatManagerRef) (.CombatantID (Utilities|Struct|BreakS_Combatant Target)) "NewEnumerator1"))
  (if _bhascondition
    (bind _total (CallFunction|DiceRoll 1 6))
    (LocalVariables|SetAttackResult (Utilities|Struct|MakeS_AttackResult true 0 0 _total))
    (LocalVariables|SetbWasAutoHit true)
    (else
      (bind _attackresult (CallFunction|ResolveAttack ActiveCombatant Target))
      (LocalVariables|SetAttackResult _attackresult)
      (LocalVariables|SetTargetCombatantCurrentHP _currenthp)
      (LocalVariables|SetTargetCombatantID _combatantid)
      (LocalVariables|SetCharacterID _characterid)
      (LocalVariables|SetTargetCombatantName _combatantname)
      (LocalVariables|SetbAttakResultHit (.bHit (Utilities|Struct|BreakS_AttackResult (LocalVariables|GetAttackResult))))
      (LocalVariables|SetAttackResultDamage (.Damage (Utilities|Struct|BreakS_AttackResult (LocalVariables|GetAttackResult))))))
  (if (LocalVariables|GetbAttakResultHit)
    (Default|ApplyDamage (Variables|Default|GetCombatManagerRef) (LocalVariables|GetTargetCombatantID) (LocalVariables|GetAttackResultDamage))
    (if (<= (- (LocalVariables|GetTargetCombatantCurrentHP) (LocalVariables|GetAttackResultDamage)) 0)
      (Utilities|FlowControl|Sequence
        (:then_0
          (Default|ApplyCondition (Variables|Default|GetCombatManagerRef) (LocalVariables|GetTargetCombatantID) "NewEnumerator10"))
        (:then_1
          (Default|SetmarkerDowned (Variables|Default|GetCombatManagerRef) (LocalVariables|GetTargetCombatantID)))
        (:then_2
          (Default|ApplyDeathtoCharacter (Variables|Default|GetPartyMangerRef) (LocalVariables|GetCharacterID))))
      (else
        (if (LocalVariables|GetbWasAutoHit)
          (Default|PostMessage (Variables|/Game/Blueprints/Combat/BP_CombatManager.BP_CombatManager_C|GetTextManagerRef (Variables|Default|GetCombatManagerRef)) (Utilities|Text|ToText(String) (Utilities|String|Append (.CombatantName (Utilities|Struct|BreakS_Combatant ActiveCombatant)) " hits for " (Utilities|String|ToString(Integer) (LocalVariables|GetAttackResultDamage)) " damage (Auto Hit)")) "NewEnumerator0")
          (else
            (Default|PostMessage (Variables|/Game/Blueprints/Combat/BP_CombatManager.BP_CombatManager_C|GetTextManagerRef (Variables|Default|GetCombatManagerRef)) (Utilities|Text|ToText(String) (Utilities|String|Append (.CombatantName (Utilities|Struct|BreakS_Combatant ActiveCombatant)) (LocalVariables|GetTargetCombatantName))) "NewEnumerator1")
            (Development|PrintString (Utilities|String|Append "CombatantID: " (Utilities|String|ToString(Integer) (LocalVariables|GetTargetCombatantID)) "Damage: " (Utilities|String|ToString(Integer) (LocalVariables|GetAttackResultDamage))))))
        (bind _bvictory (Default|CheckVictory (Variables|Default|GetCombatManagerRef)))
        (if _bvictory
          (Default|RefreshPartyPanel (Variables|Default|GetExplorationUIRef))
          (Default|EndCombat (Variables|Default|GetCombatManagerRef)))))))