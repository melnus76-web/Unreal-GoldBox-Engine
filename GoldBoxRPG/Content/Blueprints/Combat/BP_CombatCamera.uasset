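; Combat camera actor that pans and zooms over a bounded arena using Enhanced Input.
; Tick polls the pan and zoom action values, moving the actor in world XY within arena limits and adjusting spring arm length within zoom limits, both scaled by speed and delta time.
; SnapToTarget teleports the camera to a target's XY while keeping its height.
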(event EventBeginPlay)

(event Collision|EventActorBeginOverlap
  (params (OtherActor :type Actor%20Object%20Reference)))

(event EventTick
  (params (DeltaSeconds :type Float%20%28single-precision%29))
  (bind _returnvalue (Input|EnhancedActionValues|GetIA_CombatPan))
  (bind _self self)
  (bind (_x _y) (Math|Vector2D|BreakVector2D _returnvalue))
  (bind _returnvalue_2 (Transformation|GetActorLocation _self))
  (bind (_x_2 _y_2 _z) (Math|Vector|BreakVector _returnvalue_2))
  (Variables|Default|SetDelta%20Seconds DeltaSeconds)
  (Transformation|SetActorLocation self (Math|Vector|MakeVector (Math|Float|Clamp(Float) (+ _x_2 (* _x (Variables|Default|GetPanSpeed) (Variables|Default|GetDelta%20Seconds))) (Variables|Default|GetArenaMinX) (Variables|Default|GetArenaMaxX)) (Math|Float|Clamp(Float) (+ _y_2 (* _y (Variables|Default|GetPanSpeed) (Variables|Default|GetDelta%20Seconds))) (Variables|Default|GetArenaMinY) (Variables|Default|GetArenaMaxY)) _z) false true)
  (Variables|/Script/Engine.SpringArmComponent|SetTargetArmLength (Variables|Default|GetSpringArm) (Math|Float|Clamp(Float) (+ (Variables|/Script/Engine.SpringArmComponent|GetTargetArmLength (Variables|Default|GetSpringArm)) (* (* (Input|EnhancedActionValues|GetIA_CombatZoom) (Variables|Default|GetZoomSpeed)) (Variables|Default|GetDelta%20Seconds))) (Variables|Default|GetMinZoom) (Variables|Default|GetMaxZoom))))

(fn ConstructionScript)

(fn SnaptoTarget
  (params (TargetLocation :type Vector))
  (bind (_x _y) (Math|Vector|BreakVector TargetLocation))
  (Transformation|SetActorLocation (Math|Vector|MakeVector _x _y (.Z (Math|Vector|BreakVector (Transformation|GetActorLocation)))) false true))