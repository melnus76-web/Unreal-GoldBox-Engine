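; BP_CombatGrid is the tile-based combat battlefield, tracking blocked tiles and combatant occupancy by flattened tile index.
; GenerateGridFromDungeon expands a window of dungeon tiles around the player into blocks of combat tiles, blocking impassable or out-of-bounds areas.
; RebuildTileInstances renders floors and walls through instanced static meshes.
; Queries provide adjacency, square ranges, movement options, nearest free tile and radius AoE (cone and line are stubs), with spawned highlight actors.
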(event EventBeginPlay
  (bind _returnvalue (Transformation|GetActorLocation))
  (Variables|Default|SetGridOrigin _returnvalue)
  (Development|PrintString (Utilities|String|Append "BP_CombatGrid ready at: " (Utilities|String|ToString(Vector) _returnvalue)) true true "(R=0.000000,G=0.660000,B=1.000000,A=1.000000)" 5e+02)
  (CallFunction|SpawnGrid 16 16)
  (CallFunction|SetBlocked)
  (CallFunction|RebuildTileInstances)
  (Development|PrintString (Utilities|String|Append "Instances = " (Utilities|String|ToString(Integer) (Components|InstancedStaticMesh|GetInstanceCount (Variables|Default|GetTileMeshISM)))) true true "(R=0.000000,G=0.660000,B=1.000000,A=1.000000)" 2e+01))

(event Collision|EventActorBeginOverlap
  (params (OtherActor :type Actor%20Object%20Reference)))

(event EventTick
  (params (DeltaSeconds :type Float%20%28single-precision%29)))

(fn ConstructionScript)

(fn TiletoIndex
  (params (X :type Integer) (Y :type Integer))
  (return (+ X (* Y (Variables|Default|GetGridWidth)))))

(fn IndextoTile
  (params (Index :type Integer))
  (bind _gridwidth (Variables|Default|GetGridWidth))
  (return (Math|Integer|%(Integer) Index _gridwidth) (/ Index _gridwidth)))

(fn SetOccupant
  (params (X :type Integer) (Y :type Integer) (CombatantID :type Integer))
  (Utilities|Map|Add (Variables|Default|GetOccupancyMap) (CallFunction|TiletoIndex X Y) CombatantID))

(fn ClearOccupant
  (params (X :type Integer) (Y :type Integer))
  (Utilities|Map|Remove (Variables|Default|GetOccupancyMap) (CallFunction|TiletoIndex X Y)))

(fn IsOccupied
  (params (X :type Integer) (Y :type Integer))
  (return (Utilities|Map|Contains (Variables|Default|GetOccupancyMap) (CallFunction|TiletoIndex X Y))))

(fn GetOccupant
  (params (X :type Integer) (Y :type Integer))
  (bind _index (CallFunction|TiletoIndex X Y))
  (bind _occupancymap (Variables|Default|GetOccupancyMap))
  (bind (_value _returnvalue) (Utilities|Map|Find _occupancymap _index))
  (return _value _returnvalue))

(fn GetAdjacentTiles
  (params (X :type Integer) (Y :type Integer))
  ;[0.15 0.15 0.15 0.5] DY Loop
  (for _index (range -1 1)
    (LocalVariables|SetDY%20Index _index)
    ;[0.15 0.15 0.15 0.5] DX loop
    (for _index_2 (range -1 1)
      (LocalVariables|SetDX%20Index _index_2)
      (LocalVariables|SetNX%20Local (+ X (LocalVariables|GetDX%20Index)))
      (LocalVariables|SetNY%20Local (+ Y (LocalVariables|GetDY%20Index)))
      (if (not (and (== (LocalVariables|GetDY%20Index) 0) (== (LocalVariables|GetDX%20Index) 0)))
        (if (CallFunction|IsTileinBounds (LocalVariables|GetNX%20Local) (LocalVariables|GetNY%20Local))
          (Utilities|Array|Add (LocalVariables|GetAdjacentTiles) (Math|Vector2D|MakeVector2D (Math|Conversions|ToFloat(Integer) (LocalVariables|GetNX%20Local)) (Math|Conversions|ToFloat(Integer) (LocalVariables|GetNY%20Local))))))))
  (return (LocalVariables|GetAdjacentTiles)))

(fn IsTileinBounds
  (params (X :type Integer) (Y :type Integer))
  (return (Math|Boolean|ANDBoolean (>= X 0) (< X (Variables|Default|GetGridWidth)) (>= Y 0) (< Y (Variables|Default|GetGridHeight)))))

(fn SetBlocked
  (params (X :type Integer) (Y :type Integer))
  (Utilities|Set|Add (Variables|Default|GetBlockedTiles) (CallFunction|TiletoIndex X Y)))

(fn IsBlocked
  (params (X :type Integer) (Y :type Integer))
  (return (Utilities|Set|Contains (Variables|Default|GetBlockedTiles) (CallFunction|TiletoIndex X Y))))

(fn IsTraversable
  (params (X :type Integer) (Y :type Integer))
  (return (Math|Boolean|ANDBoolean (CallFunction|IsTileinBounds X Y) (not (CallFunction|IsBlocked X Y)) (not (CallFunction|IsOccupied X Y)))))

(fn GetTilesinRange
  (params (OriginX :type Integer) (OriginY :type Integer) (Range :type Integer))
  (LocalVariables|SetRange-1 (* Range -1))
  ;[0.15 0.15 0.15 0.5] DX Loop (Outer)
  (for _index (range (LocalVariables|GetRange-1) Range)
    (LocalVariables|SetDX%20Index _index)
    ;[0.15 0.15 0.15 0.5] DY Loop (Inner)
    (for _index_2 (range (LocalVariables|GetRange-1) Range)
      (LocalVariables|SetDY%20Index _index_2)
      (LocalVariables|SetNX%20Local (+ OriginX (LocalVariables|GetDX%20Index)))
      (LocalVariables|SetNY%20Local (+ OriginY (LocalVariables|GetDY%20Index)))
      (if (CallFunction|IsTileinBounds (LocalVariables|GetNX%20Local) (LocalVariables|GetNY%20Local))
        (Utilities|Array|Add (LocalVariables|GetRangeTiles) (Math|Vector2D|MakeVector2D (Math|Conversions|ToFloat(Integer) (LocalVariables|GetNX%20Local)) (Math|Conversions|ToFloat(Integer) (LocalVariables|GetNY%20Local)))))))
  (return (LocalVariables|GetRangeTiles)))

(fn GetTilesinSpellAoE
  (params (OriginX :type Integer) (OriginY :type Integer) (Shape :type E_AoEShape%20Enum :default "NewEnumerator0") (Size :type Integer))
  (switch Utilities|FlowControl|Switch|SwitchonE_AoEShape Shape
    (:NewEnumerator0
      (return (LocalVariables|GetAoETiles)))
    (:NewEnumerator1
      (bind _output_get (LocalVariables|SetAoETiles (CallFunction|GetTilesinRange OriginX OriginY Size)))
      (return _output_get))
    (:NewEnumerator2
      ;[0.15 0.15 0.15 0.5] TODO: GB-047/GB-051: Implement Cone and Line Shapes
      (Development|PrintString "GetTilesInDpellAoE:: Cone not implemented (Phase 8)"))
    (:NewEnumerator3
      (Development|PrintString "GetTilesInDpellAoE:: Line not implemented (Phase 8)"))))

(fn TiletoWorld
  (params (X :type Integer) (Y :type Integer))
  (bind _tilesize (Variables|Default|GetTileSize))
  (bind _returnvalue (/ _tilesize 2.0))
  (return (+ (Math|Vector|MakeVector (+ (* X _tilesize) _returnvalue) (+ _returnvalue (* Y _tilesize)) 0.0) (Variables|Default|GetGridOrigin))))

(fn SpawnGrid
  (params (Width :type Integer) (Height :type Integer))
  (Variables|Default|SetGridWidth Width)
  (Variables|Default|SetGridHeight Height)
  (Utilities|Map|Clear (Variables|Default|GetOccupancyMap))
  (Utilities|Set|Clear (Variables|Default|GetBlockedTiles))
  (CallFunction|RebuildTileInstances))

(fn RebuildTileInstances
  (bind _tilesize (Variables|Default|GetTileSize))
  (bind _returnvalue (/ _tilesize 1e+02))
  (bind _returnvalue_2 (* _returnvalue 0.95))
  (Components|InstancedStaticMesh|ClearInstances (Variables|Default|GetTileMeshISM))
  (Components|InstancedStaticMesh|ClearInstances (Variables|Default|GetWallMeshISM))
  (Utilities|Map|Clear (Variables|Default|GetTileIndexToInstanceIndex))
  ;[0.15 0.15 0.15 0.5] Y Loop (Outer)
  (for _index (range 0 (- (Variables|Default|GetGridHeight) 1))
    (LocalVariables|SetY%20Loop%20Index _index)
    ;[0.15 0.15 0.15 0.5] X Loop (Inner)
    (for _index_2 (range 0 (- (Variables|Default|GetGridWidth) 1))
      (LocalVariables|SetX%20Loop%20Index _index_2)
      (if (CallFunction|IsBlocked (LocalVariables|GetX%20Loop%20Index) (LocalVariables|GetY%20Loop%20Index))
        (Components|InstancedStaticMesh|AddInstance (Variables|Default|GetWallMeshISM) (Math|Transform|MakeTransform (CallFunction|TiletoWorld (LocalVariables|GetX%20Loop%20Index) (LocalVariables|GetY%20Loop%20Index)) "0, 0, 0" "2.000000,2.000000,2.000000") true)
        (else
          (bind _returnvalue_3 (Components|InstancedStaticMesh|AddInstance (Variables|Default|GetTileMeshISM) (Math|Transform|MakeTransform (CallFunction|TiletoWorld (LocalVariables|GetX%20Loop%20Index) (LocalVariables|GetY%20Loop%20Index)) "0, 0, 0" (Math|Vector|MakeVector _returnvalue_2 _returnvalue_2 1.0)) true))
          (Utilities|Map|Add (Variables|Default|GetTileIndexToInstanceIndex) (CallFunction|TiletoIndex (LocalVariables|GetX%20Loop%20Index) (LocalVariables|GetY%20Loop%20Index)) _returnvalue_3))))))

(fn GenerateGridfromDungeon
  (params (PlayerTileX :type Integer) (PlayerTileY :type Integer))
  (bind _mapmanagerref (Variables|Default|GetMapManagerRef))
  (bind _currentmap (Variables|/Game/Blueprints/Dungeon/BP_MapManager.BP_MapManager_C|GetCurrentMap _mapmanagerref))
  (bind (_levelid _width _height) (Utilities|Struct|BreakS_DungeonMap _currentmap))
  (LocalVariables|SetWindowOriginX (- PlayerTileX 1))
  (LocalVariables|SetWindowOriginY (- PlayerTileY 1))
  (CallFunction|SpawnGrid 16 16)
  ;[0.15 0.15 0.15 0.5] DY Loop (Outer)
  (for _index (range 0 3)
    (LocalVariables|SetDY%20LoopIndex _index)
    ;[0.15 0.15 0.15 0.5] DX Loop (Inner)
    (for _index_2 (range 0 3)
      (LocalVariables|SetDXLoopIndex _index_2)
      (LocalVariables|SetDungeonX (+ (LocalVariables|GetWindowOriginX) (LocalVariables|GetDXLoopIndex)))
      (LocalVariables|SetDungeonY (+ (LocalVariables|GetWindowOriginY) (LocalVariables|GetDY%20LoopIndex)))
      (LocalVariables|SetbNotPassable (not (.Passable (Utilities|Struct|BreakS_DungeonTile (Default|GetTile _mapmanagerref (LocalVariables|GetDungeonX) (LocalVariables|GetDungeonY))))))
      (LocalVariables|SetbOutOfBounds (not (Math|Boolean|ANDBoolean (>= (LocalVariables|GetDungeonX) 0) (< (LocalVariables|GetDungeonX) _width) (>= (LocalVariables|GetDungeonY) 0) (< (LocalVariables|GetDungeonY) _height))))
      (if (or (LocalVariables|GetbNotPassable) (LocalVariables|GetbOutOfBounds))
        ;[0.15 0.15 0.15 0.5] SY Loop (Outer)
        (for _index_3 (range 0 3)
          (LocalVariables|SetSYIndex _index_3)
          ;[0.15 0.15 0.15 0.5] SX Loop (Inner)
          (for _index_4 (range 0 3)
            (LocalVariables|SetSXIndex _index_4)
            (CallFunction|SetBlocked (+ (* (LocalVariables|GetDXLoopIndex) 4) (LocalVariables|GetSXIndex)) (+ (* (LocalVariables|GetDY%20LoopIndex) 4) (LocalVariables|GetSYIndex))))))))
  (CallFunction|RebuildTileInstances))

(fn FindNearestTraverrsableTile
  (params (PreferredX :type Integer) (PreferredY :type Integer))
  (if (CallFunction|IsTraversable PreferredX PreferredY)
    (LocalVariables|SetResultX PreferredX)
    (LocalVariables|SetResultY PreferredY)
    (LocalVariables|SetbResultFound true)
    (return (LocalVariables|GetResultX) (LocalVariables|GetResultY) (LocalVariables|GetbResultFound))
    (else
      ;[0.15 0.15 0.15 0.5] Outer Loop
      (for _index (range 0 (LocalVariables|GetRange))
        (if (not (LocalVariables|GetbResultFound))
          ;[0.15 0.15 0.15 0.5] Inner Loop
          (for _array_element (CallFunction|GetTilesinRange PreferredX PreferredY _index)
            (if (not (LocalVariables|GetbResultFound))
              (LocalVariables|SetTileX (Math|Float|Truncate (.X (Math|Vector2D|BreakVector2D _array_element))))
              (LocalVariables|SetTileY (Math|Float|Truncate (.Y (Math|Vector2D|BreakVector2D _array_element))))
              (if (CallFunction|IsTraversable (LocalVariables|GetTileX) (LocalVariables|GetTileY))
                (if (not (CallFunction|IsOccupied (LocalVariables|GetTileX) (LocalVariables|GetTileY)))
                  (LocalVariables|SetResultX (LocalVariables|GetTileX))
                  (LocalVariables|SetResultY (LocalVariables|GetTileY))
                  (LocalVariables|SetbResultFound true)))))))
      (return (LocalVariables|GetResultX) (LocalVariables|GetResultY) (LocalVariables|GetbResultFound)))))

(fn HighlightTiles
  (params (Tiles :type Array%20of%20Vector%202D%20Structures) (Colour :type Linear%20Color%20Structure))
  (Utilities|Array|Clear (Variables|Default|GetSpawnedHighlights))
  (for _array_element Tiles
    (bind _returnvalue (Game|SpawnActorfromClass "/Game/Blueprints/Combat/BP_TileHighlight.BP_TileHighlight_C" (Math|Transform|MakeTransform (Math|Vector|MakeVector (.x (CallFunction|TiletoWorld (Math|Float|Truncate (.X (Math|Vector2D|BreakVector2D _array_element))) (Math|Float|Truncate (.Y (Math|Vector2D|BreakVector2D _array_element))))) (.y (CallFunction|TiletoWorld (Math|Float|Truncate (.X (Math|Vector2D|BreakVector2D _array_element))) (Math|Float|Truncate (.Y (Math|Vector2D|BreakVector2D _array_element))))) 5.0) "0, 0, 0" "1.000000,1.000000,1.000000") "Undefined" "MultiplyWithRoot" 0 0))
    (Default|Initialise _returnvalue Colour)
    (Utilities|Array|Add (Variables|Default|GetSpawnedHighlights) _returnvalue)))

(fn ClearHighlights
  (for _array_element (Variables|Default|GetSpawnedHighlights)
    (Actor|DestroyActor _array_element))
  (Utilities|Array|Clear (Variables|Default|GetSpawnedHighlights)))

(fn GetValidMoveTiles
  (params (OriginX :type Integer) (OriginY :type Integer) (Range :type Integer))
  (for _array_element (CallFunction|GetTilesinRange OriginX OriginY Range)
    (LocalVariables|SetBreakX (.X (Math|Vector2D|BreakVector2D _array_element)))
    (LocalVariables|SetBreakY (.Y (Math|Vector2D|BreakVector2D _array_element)))
    (LocalVariables|SetTileX (Math|Float|Truncate (LocalVariables|GetBreakX)))
    (LocalVariables|SetTileY (Math|Float|Truncate (LocalVariables|GetBreakY)))
    (if (CallFunction|IsTraversable (LocalVariables|GetTileX) (LocalVariables|GetTileY))
      (if (not (CallFunction|IsOccupied (LocalVariables|GetTileX) (LocalVariables|GetTileY)))
        (Utilities|Array|Add (LocalVariables|GetFilteredTiles) (Math|Vector2D|MakeVector2D (LocalVariables|GetBreakX) (LocalVariables|GetBreakY))))))
  (return (LocalVariables|GetFilteredTiles)))