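; BP_CombatantMarker is a labelled, clickable world marker representing a combatant in combat, either a monster or a non-monster.
; Initialise sets the name label and swaps the mesh to a red cone for monsters or a smaller green cube otherwise, tinting it through a dynamic material instance.
; Clicking the mesh checks the game instance's CombatManager for active target selection, then only prints debug text according to the monster flag.
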(event OnClicked(MarkerMesh)
  (params (TouchedComponent :type Primitive%20Component%20Object%20Reference) (ButtonPressed :type Key%20Structure :default "None"))
  (bind _asbp_game_manager (Utilities|Casting|CastToBP_GameManager (Game|GetGameInstance)))
  (if (Variables|/Game/Blueprints/Combat/BP_CombatManager.BP_CombatManager_C|GetbSelectingTarget (Variables|/Game/Blueprints/Core/BP_GameManager.BP_GameManager_C|GetCombatManager _asbp_game_manager))
    (if (Variables|Default|GetbIsMonster)
      (Development|PrintString "Marker ClickedHello" true true "(R=0.000000,G=0.660000,B=1.000000,A=1.000000)" 5e+01)
      (else
        (Development|PrintString "Is Monster - false")))))

(event EventBeginPlay)

(event Collision|EventActorBeginOverlap
  (params (OtherActor :type Actor%20Object%20Reference)))

(event EventTick
  (params (DeltaSeconds :type Float%20%28single-precision%29)))

(fn ConstructionScript)

(fn Initialise
  (params (InCombatantName :type String) (bInIsMonster :type Boolean))
  (Rendering|Components|TextRender|SetText (Variables|Default|GetMarkerLabel) (Utilities|Text|ToText(String) InCombatantName))
  (bind _output_get (Variables|Default|SetbIsMonster bInIsMonster))
  (if _output_get
    (Components|StaticMesh|SetStaticMesh (Variables|Default|GetMarkerMesh) "/Engine/BasicShapes/Cone.Cone")
    (bind _returnvalue (Rendering|Material|CreateDynamicMaterialInstance (Variables|Default|GetMarkerMesh) 0 "/Game/Art/Materials/M_CombatantMarker.M_CombatantMarker" "None" :!class /Script/Engine.PrimitiveComponent))
    (Rendering|Material|SetVectorParameterValue _returnvalue "MarkerColour" (Utilities|Struct|MakeLinearColor 1.0 0.0 0.0 1.0) :!class /Script/Engine.MaterialInstanceDynamic)
    (Transformation|SetWorldScale3D (Variables|Default|GetMarkerMesh) "1.000000,1.000000,1.000000")
    (else
      (Components|StaticMesh|SetStaticMesh (Variables|Default|GetMarkerMesh) "/Engine/BasicShapes/Cube.Cube")
      (bind _returnvalue_2 (Rendering|Material|CreateDynamicMaterialInstance (Variables|Default|GetMarkerMesh) 0 "/Game/Art/Materials/M_CombatantMarker.M_CombatantMarker" "None" :!class /Script/Engine.PrimitiveComponent))
      (Rendering|Material|SetVectorParameterValue _returnvalue_2 "MarkerColour" (Utilities|Struct|MakeLinearColor 0.0 1.0 0.0 1.0) :!class /Script/Engine.MaterialInstanceDynamic)
      (Transformation|SetWorldScale3D (Variables|Default|GetMarkerMesh) "0.800000,0.800000,0.800000"))))