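; Combat resolver Blueprint for grid-based, party-versus-monster fights, handling attacks, damage, conditions and victory/defeat checks.
; ExecutePlayerAttack checks range, helpless targets and class-based ambush bonuses, then loops ResolveSingleAttack for damage, death, morale and messages.
; Helpers rebuild Combatant structs to write back changes, sync party HP to PartyManager and tick poison saves.
; As wired, WasAutoHit only changes hit messages, and ProcessAttackOutcome always ends combat.
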(event EventBeginPlay)

(event Collision|EventActorBeginOverlap
  (params (OtherActor :type Actor%20Object%20Reference)))

(event EventTick
  (params (DeltaSeconds :type Float%20%28single-precision%29)))

(fn ConstructionScript)

(fn HasCondition
  (params (CombatantID :type Integer) (ConditionCheck :type E_Condition%20Enum :default "NewEnumerator0"))
  (bind _combatants (Variables|Default|GetCombatants))
  (bind (_combatant _bfound) (CallFunction|FindCombatantbyID _combatants CombatantID))
  (if _bfound
    (return (Utilities|Array|ContainsItem (.Conditions (Utilities|Struct|BreakS_Combatant _combatant)) ConditionCheck))
    (else
      (return false))))

(fn IsCombatantIncapacitated
  (params (CombatantID :type Integer))
  (bind _bhascondition (CallFunction|HasCondition CombatantID "NewEnumerator10"))
  (bind _bhascondition_2 (CallFunction|HasCondition CombatantID "NewEnumerator2"))
  (bind _bhascondition_3 (CallFunction|HasCondition CombatantID "NewEnumerator11"))
  (bind _bhascondition_4 (CallFunction|HasCondition CombatantID "NewEnumerator10"))
  (return (Math|Boolean|ORBoolean _bhascondition _bhascondition_2 _bhascondition_3 _bhascondition_4)))

(fn ApplyDamage
  (params (CombatantID :type Integer) (Damage :type Integer))
  (bind _combatants (Variables|Default|GetCombatants))
  (bind (_combatant _bfound) (CallFunction|FindCombatantbyID _combatants CombatantID))
  (bind (_combatantid _combatantname _isplayercontrolled _sourcecharacter _sourcemonster _ismonster _gridposition _currenthp _maxhp _defenserating _strikenumber _initiative _actionsremaining _movementrange _attacksremaining _hasactedthisround _conditions _tilesmovedthisturn _characterid) (Utilities|Struct|BreakS_Combatant _combatant))
  (if _bfound
    (LocalVariables|SetNewHP (- _currenthp Damage))
    (if _ismonster
      _
      (else
        (Default|UpdateCharacterHP (Variables|Default|GetPartyManagerRef) _characterid (LocalVariables|GetNewHP))))
    (for (_array_element _array_index) (Variables|Default|GetCombatants)
      (if (== (.CombatantID (Utilities|Struct|BreakS_Combatant _array_element)) CombatantID)
        (Utilities|Array|SetArrayElem (Variables|Default|GetCombatants) _array_index (Utilities|Struct|MakeS_Combatant (.CombatantID (Utilities|Struct|BreakS_Combatant _array_element)) (.CombatantName (Utilities|Struct|BreakS_Combatant _array_element)) (.IsPlayerControlled (Utilities|Struct|BreakS_Combatant _array_element)) (.SourceCharacter (Utilities|Struct|BreakS_Combatant _array_element)) (.SourceMonster (Utilities|Struct|BreakS_Combatant _array_element)) (.IsMonster (Utilities|Struct|BreakS_Combatant _array_element)) (.GridPosition (Utilities|Struct|BreakS_Combatant _array_element)) (LocalVariables|GetNewHP) (.MaxHP (Utilities|Struct|BreakS_Combatant _array_element)) (.DefenseRating (Utilities|Struct|BreakS_Combatant _array_element)) (.StrikeNumber (Utilities|Struct|BreakS_Combatant _array_element)) (.Initiative (Utilities|Struct|BreakS_Combatant _array_element)) (.ActionsRemaining (Utilities|Struct|BreakS_Combatant _array_element)) (.MovementRange (Utilities|Struct|BreakS_Combatant _array_element)) (.AttacksRemaining (Utilities|Struct|BreakS_Combatant _array_element)) (.HasActedThisRound (Utilities|Struct|BreakS_Combatant _array_element)) (.Conditions (Utilities|Struct|BreakS_Combatant _array_element)) (.TilesMovedThisTurn (Utilities|Struct|BreakS_Combatant _array_element)) (.CharacterID (Utilities|Struct|BreakS_Combatant _array_element)) (.MoraleState (Utilities|Struct|BreakS_Combatant _array_element)) (.GroupID (Utilities|Struct|BreakS_Combatant _array_element)) (.AttackRange (Utilities|Struct|BreakS_Combatant _array_element))))))))

(fn ApplyCondition
  (params (CombatantID :type Integer) (NewCondition :type E_Condition%20Enum :default "NewEnumerator0"))
  (bind _combatants (Variables|Default|GetCombatants))
  (bind (_combatant _bfound) (CallFunction|FindCombatantbyID _combatants CombatantID))
  (bind _conditions (Utilities|Struct|BreakS_Combatant _combatant))
  (if _bfound
    (Utilities|Array|Add _conditions NewCondition)
    (bind (_array_element _array_index) (Utilities|Array|ForEachLoopwithBreak (Variables|Default|GetCombatants) :!label _label)
      (:LoopBody
        (if (== (.CombatantID (Utilities|Struct|BreakS_Combatant _array_element)) CombatantID)
          (Utilities|Array|SetArrayElem (Variables|Default|GetCombatants) _array_index (Utilities|Struct|MakeS_Combatant (.CombatantID (Utilities|Struct|BreakS_Combatant _array_element)) (.CombatantName (Utilities|Struct|BreakS_Combatant _array_element)) (.IsPlayerControlled (Utilities|Struct|BreakS_Combatant _array_element)) (.SourceCharacter (Utilities|Struct|BreakS_Combatant _array_element)) (.SourceMonster (Utilities|Struct|BreakS_Combatant _array_element)) (.IsMonster (Utilities|Struct|BreakS_Combatant _array_element)) (.GridPosition (Utilities|Struct|BreakS_Combatant _array_element)) (.CurrentHP (Utilities|Struct|BreakS_Combatant _array_element)) (.MaxHP (Utilities|Struct|BreakS_Combatant _array_element)) (.DefenseRating (Utilities|Struct|BreakS_Combatant _array_element)) (.StrikeNumber (Utilities|Struct|BreakS_Combatant _array_element)) (.Initiative (Utilities|Struct|BreakS_Combatant _array_element)) (.ActionsRemaining (Utilities|Struct|BreakS_Combatant _array_element)) (.MovementRange (Utilities|Struct|BreakS_Combatant _array_element)) (.AttacksRemaining (Utilities|Struct|BreakS_Combatant _array_element)) (.HasActedThisRound (Utilities|Struct|BreakS_Combatant _array_element)) _conditions (.TilesMovedThisTurn (Utilities|Struct|BreakS_Combatant _array_element)) (.CharacterID (Utilities|Struct|BreakS_Combatant _array_element)) (.MoraleState (Utilities|Struct|BreakS_Combatant _array_element)) (.GroupID (Utilities|Struct|BreakS_Combatant _array_element)) (.AttackRange (Utilities|Struct|BreakS_Combatant _array_element))))
          (goto _label Break))))))

(fn ConditiontoRemove
  (params (CombatantID :type Integer) (ConditionToRemove :type E_Condition%20Enum :default "NewEnumerator0"))
  (bind _combatants (Variables|Default|GetCombatants))
  (bind (_combatant _bfound) (CallFunction|FindCombatantbyID _combatants CombatantID))
  (bind _conditions (Utilities|Struct|BreakS_Combatant _combatant))
  (if _bfound
    (Utilities|Array|RemoveItem _conditions ConditionToRemove)
    (bind (_array_element _array_index) (Utilities|Array|ForEachLoopwithBreak (Variables|Default|GetCombatants) :!label _label)
      (:LoopBody
        (if (== (.CombatantID (Utilities|Struct|BreakS_Combatant _array_element)) CombatantID)
          (Utilities|Array|SetArrayElem (Variables|Default|GetCombatants) _array_index (Utilities|Struct|MakeS_Combatant (.CombatantID (Utilities|Struct|BreakS_Combatant _array_element)) (.CombatantName (Utilities|Struct|BreakS_Combatant _array_element)) (.IsPlayerControlled (Utilities|Struct|BreakS_Combatant _array_element)) (.SourceCharacter (Utilities|Struct|BreakS_Combatant _array_element)) (.SourceMonster (Utilities|Struct|BreakS_Combatant _array_element)) (.IsMonster (Utilities|Struct|BreakS_Combatant _array_element)) (.GridPosition (Utilities|Struct|BreakS_Combatant _array_element)) (.CurrentHP (Utilities|Struct|BreakS_Combatant _array_element)) (.MaxHP (Utilities|Struct|BreakS_Combatant _array_element)) (.DefenseRating (Utilities|Struct|BreakS_Combatant _array_element)) (.StrikeNumber (Utilities|Struct|BreakS_Combatant _array_element)) (.Initiative (Utilities|Struct|BreakS_Combatant _array_element)) (.ActionsRemaining (Utilities|Struct|BreakS_Combatant _array_element)) (.MovementRange (Utilities|Struct|BreakS_Combatant _array_element)) (.AttacksRemaining (Utilities|Struct|BreakS_Combatant _array_element)) (.HasActedThisRound (Utilities|Struct|BreakS_Combatant _array_element)) _conditions (.TilesMovedThisTurn (Utilities|Struct|BreakS_Combatant _array_element)) (.CharacterID (Utilities|Struct|BreakS_Combatant _array_element)) (.MoraleState (Utilities|Struct|BreakS_Combatant _array_element)) (.GroupID (Utilities|Struct|BreakS_Combatant _array_element)) (.AttackRange (Utilities|Struct|BreakS_Combatant _array_element))))
          (goto _label Break))))))

(fn TickConditions
  (params (CombatantID :type Integer))
  (bind _combatants (Variables|Default|GetCombatants))
  (bind (_combatant _bfound) (CallFunction|FindCombatantbyID _combatants CombatantID))
  (bind (_combatantid _combatantname _isplayercontrolled _sourcecharacter _sourcemonster _ismonster _gridposition _currenthp _maxhp _defenserating _strikenumber _initiative _actionsremaining _movementrange _attacksremaining _hasactedthisround _conditions) (Utilities|Struct|BreakS_Combatant _combatant))
  (if _bfound
    (LocalVariables|SetConditions _conditions)
    (LocalVariables|SetCharacter _sourcecharacter)
    (LocalVariables|SetCombatantName _combatantname)
    (for _array_element (LocalVariables|GetConditions)
      (switch Utilities|FlowControl|Switch|SwitchonE_Condition _array_element
        (:NewEnumerator3
          (bind _bsuccess (CallFunction|ResolveSave (LocalVariables|GetCharacter) "NewEnumerator5"))
          (if _bsuccess
            (Default|PostMessage (Variables|Default|GetTextManagerRef) (Utilities|Text|ToText(String) (CallFunction|FormatPoisonResistMessage (LocalVariables|GetCombatantName))) "NewEnumerator1")
            (else
              (bind _total (CallFunction|DiceRoll 1 4))
              (CallFunction|ApplyDamage CombatantID _total)
              (Default|PostMessage (Variables|Default|GetTextManagerRef) (Utilities|Text|ToText(String) (CallFunction|FormatPoisonDamage (LocalVariables|GetCombatantName) _total)) "NewEnumerator1"))))))))

(fn ProcessAttackOutcome
  (params (Attacker :type S%20Combatant%20Structure) (Defender :type S%20Combatant%20Structure))
  (Default|CheckVictory (Variables|Default|GetCombatManagerRef))
  (if true
    (Default|EndCombat (Variables|Default|GetCombatManagerRef) true)
    (else
      (Default|OnActionComplete (Variables|Default|GetCombatManagerRef)))))

(fn ResolveSingleAttack
  (params (Attacker :type S%20Combatant%20Structure) (Defender :type S%20Combatant%20Structure) (bWasAutoHit :type Boolean) (AmbushMultiplier :type Integer) (AmbushSituational :type Integer) (bRerollOnes :type Boolean))
  (bind (_combatantid _combatantname) (Utilities|Struct|BreakS_Combatant Defender))
  (LocalVariables|SetAttackerName (.CombatantName (Utilities|Struct|BreakS_Combatant Attacker)))
  (LocalVariables|SetDefenderID _combatantid)
  (LocalVariables|SetDefenderName _combatantname)
  (if (not (CallFunction|HasCondition (LocalVariables|GetDefenderID) "NewEnumerator10"))
    (bind _attackresult (CallFunction|ResolveAttack Attacker Defender AmbushSituational))
    (if (.bHit (Utilities|Struct|BreakS_AttackResult _attackresult))
      (LocalVariables|SetDamageRoll (* AmbushMultiplier (.Damage (Utilities|Struct|BreakS_AttackResult _attackresult))))
      (if bRerollOnes
        (LocalVariables|SetFinalDamage (CallFunction|RerollOnesonDamage (LocalVariables|GetDamageRoll)))
        (else
          (LocalVariables|SetFinalDamage (LocalVariables|GetDamageRoll))))
      (CallFunction|ApplyDamage (LocalVariables|GetDefenderID) (LocalVariables|GetFinalDamage))
      (if (<= (.CurrentHP (Utilities|Struct|BreakS_Combatant (.Combatant (CallFunction|FindCombatantbyID (Variables|Default|GetCombatants) (LocalVariables|GetDefenderID))))) 0)
        (Default|PostMessage (Variables|Default|GetTextManagerRef) (Utilities|Text|ToText(String) (CallFunction|FormatDefeatMessage (LocalVariables|GetDefenderName))) "NewEnumerator1")
        (CallFunction|ApplyCondition (LocalVariables|GetDefenderID) "NewEnumerator10")
        (Default|RemoveMarkerforCombatant (Variables|Default|GetCombatManagerRef) (LocalVariables|GetDefenderID))
        (Default|ResolveMorale (Variables|Default|GetCombatManagerRef) (.GroupID (Utilities|Struct|BreakS_Combatant (.Combatant (CallFunction|FindCombatantbyID (Variables|Default|GetCombatants) (LocalVariables|GetDefenderID)))))))
      (if bWasAutoHit
        (Default|PostMessage (Variables|Default|GetTextManagerRef) (Utilities|Text|ToText(String) (CallFunction|FormatAutoHitMessage (LocalVariables|GetAttackerName) (LocalVariables|GetDefenderName) (LocalVariables|GetFinalDamage))) "NewEnumerator1")
        (else
          (Default|PostMessage (Variables|Default|GetTextManagerRef) (Utilities|Text|ToText(String) (CallFunction|FormatHitMessage (LocalVariables|GetAttackerName) (LocalVariables|GetFinalDamage) (.RollResult (Utilities|Struct|BreakS_AttackResult _attackresult)) (.RollNeeded (Utilities|Struct|BreakS_AttackResult _attackresult)))) "NewEnumerator1")))
      (else
        (Default|PostMessage (Variables|Default|GetTextManagerRef) (Utilities|Text|ToText(String) (CallFunction|FormatMissMessage (LocalVariables|GetAttackerName) (.RollResult (Utilities|Struct|BreakS_AttackResult _attackresult)) (.RollNeeded (Utilities|Struct|BreakS_AttackResult _attackresult)))) "NewEnumerator1")))))

(fn ExecutePlayerAttack
  (params (TargetCombatantID :type Integer))
  (bind _combatants (Variables|Default|GetCombatants))
  (bind _combatants_2 (Variables|Default|GetCombatants))
  (bind _combatmanagerref (Variables|Default|GetCombatManagerRef))
  (bind (_combatant _bfound) (CallFunction|FindCombatantbyID _combatants TargetCombatantID))
  (bind _currentcombatantid (Variables|/Game/Blueprints/Combat/BP_CombatManager.BP_CombatManager_C|GetCurrentCombatantID _combatmanagerref))
  (bind (_combatantid _combatantname) (Utilities|Struct|BreakS_Combatant _combatant))
  (bind _combatant_2 (CallFunction|FindCombatantbyID _combatants_2 _currentcombatantid))
  (Variables|/Game/Blueprints/Combat/BP_CombatManager.BP_CombatManager_C|SetbSelectingTarget (Variables|Default|GetCombatManagerRef) false)
  (if _bfound
    (LocalVariables|SetDefenderCombatant _combatant)
    (LocalVariables|SetDefenderName _combatantname)
    (LocalVariables|SetDefendantID _combatantid)
    (Utilities|FlowControl|Sequence
      (:then_0
        (LocalVariables|SetAttackerCombatant _combatant_2)
        (LocalVariables|SetAttackerName (.CombatantName (Utilities|Struct|BreakS_Combatant _combatant_2))))
      (:then_1
        (if (<= (CallFunction|GetCombatDistance (.GridPosition (Utilities|Struct|BreakS_Combatant (LocalVariables|GetAttackerCombatant))) (.GridPosition (Utilities|Struct|BreakS_Combatant (LocalVariables|GetDefenderCombatant)))) (.AttackRange (Utilities|Struct|BreakS_Combatant (LocalVariables|GetAttackerCombatant))))
          (if (Math|Boolean|ORBoolean (CallFunction|HasCondition (LocalVariables|GetDefendantID) "NewEnumerator1") (CallFunction|HasCondition (LocalVariables|GetDefendantID) "NewEnumerator2") (CallFunction|HasCondition (LocalVariables|GetDefendantID) "NewEnumerator11"))
            (LocalVariables|SetbWasAutoHit true)
            (elif (or (Utilities|Enum|Equal(Enum) (.Class1 (Utilities|Struct|BreakS_Character (.SourceCharacter (Utilities|Struct|BreakS_Combatant (LocalVariables|GetAttackerCombatant))))) "NewEnumerator7") (Utilities|Enum|Equal(Enum) (.Class2 (Utilities|Struct|BreakS_Character (.SourceCharacter (Utilities|Struct|BreakS_Combatant (LocalVariables|GetAttackerCombatant))))) "NewEnumerator7"))
              (bind _bflanked (CallFunction|IsFlanked (.GridPosition (Utilities|Struct|BreakS_Combatant (LocalVariables|GetDefenderCombatant))) (Variables|Default|GetCombatants) (LocalVariables|GetDefendantID)))
              (if (or _bflanked (> (.SkillHideInShadows (Utilities|Struct|BreakS_Character (.SourceCharacter (Utilities|Struct|BreakS_Combatant (LocalVariables|GetAttackerCombatant))))) 50))
                (LocalVariables|SetAmbushSituational 4)
                (bind _multiplier (CallFunction|GetAmbushMultiplier (.Level (Utilities|Struct|BreakS_Character (.SourceCharacter (Utilities|Struct|BreakS_Combatant (LocalVariables|GetAttackerCombatant)))))))
                (LocalVariables|SetAmbushMultiplier _multiplier))))
          (LocalVariables|SetAttacksThisRound (.AttacksThisRound (CallFunction|GetAttacksThisRound (LocalVariables|GetAttackerCombatant))))
          (LocalVariables|SetbRerollOnes (.bRerollOnes (CallFunction|GetAttacksThisRound (LocalVariables|GetAttackerCombatant))))
          (for _index (range 0 (- (LocalVariables|GetAttacksThisRound) 1))
            (CallFunction|ResolveSingleAttack (LocalVariables|GetAttackerCombatant) (LocalVariables|GetDefenderCombatant) (LocalVariables|GetbWasAutoHit) (LocalVariables|GetAmbushMultiplier) (LocalVariables|GetAmbushSituational) (LocalVariables|GetbRerollOnes)))
          (CallFunction|ProcessAttackOutcome (LocalVariables|GetAttackerCombatant) (LocalVariables|GetDefenderCombatant))
          (else
            (Default|PostMessage (Variables|Default|GetTextManagerRef) (Utilities|Text|ToText(String) (Utilities|String|Append (LocalVariables|GetAttackerName) " is out of range")) "NewEnumerator1")
            (Default|OnActionComplete (Variables|Default|GetCombatManagerRef))))))))

(fn CheckVictory
  (LocalVariables|SetbAllEnemiesDead true)
  (for _array_element (Variables|Default|GetCombatants)
    (if (.IsMonster (Utilities|Struct|BreakS_Combatant _array_element))
      (if (not (CallFunction|HasCondition (.CombatantID (Utilities|Struct|BreakS_Combatant _array_element)) "NewEnumerator10"))
        (LocalVariables|SetbAllEnemiesDead false))))
  (return (LocalVariables|GetbAllEnemiesDead)))

(fn CheckDefeat
  (LocalVariables|SetbAllPartyDead true)
  (for _array_element (Variables|Default|GetCombatants)
    (LocalVariables|SetLocalCombatantID (.CombatantID (Utilities|Struct|BreakS_Combatant _array_element)))
    (if (== (.IsMonster (Utilities|Struct|BreakS_Combatant _array_element)) false)
      (if (not (CallFunction|HasCondition (LocalVariables|GetLocalCombatantID) "NewEnumerator10"))
        (LocalVariables|SetbAllPartyDead false))))
  (return (LocalVariables|GetbAllPartyDead)))