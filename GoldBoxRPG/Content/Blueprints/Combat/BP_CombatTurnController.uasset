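; Turn controller for grid-based combat that sequences player and enemy turns and counts rounds.
; Rolls a d10 initiative per combatant and orders them lowest first, then advances through that order, skipping incapacitated combatants with a loop safety counter.
; Each advance ticks conditions through the combat manager, then either opens player input or passes the combatant to the enemy AI.
; Player turn start rebuilds the combatant struct in both local and manager arrays.
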(event EventBeginPlay)

(event Collision|EventActorBeginOverlap
  (params (OtherActor :type Actor%20Object%20Reference)))

(event EventTick
  (params (DeltaSeconds :type Float%20%28single-precision%29)))

(fn ConstructionScript)

(fn FindActiveCombatant
  (bind _combatants (Variables|Default|GetCombatants))
  (bind _currentcombatantid (Variables|Default|GetCurrentCombatantID))
  (bind (_combatant _bfound) (CallFunction|FindCombatantbyID _combatants _currentcombatantid))
  (if _bfound
    (return true (.IsPlayerControlled (Utilities|Struct|BreakS_Combatant _combatant)))))

(fn FinishEnemyTurn
  (CallFunction|OnActionComplete))

(fn OnActionComplete
  (bind _bisfound (CallFunction|FindActiveCombatant))
  (if _bisfound
    (CallFunction|AdvancetoNextCombatant)
    (CallFunction|DispatchTurn (Variables|Default|GetCurrentCombatantID))
    (else
      (Development|PrintString "OnActionComplete: No active combatant found" true true "(R=1.000000,G=0.000021,B=0.000000,A=1.000000)" 1e+02))))

(fn AdvancetoNextCombatant
  (LocalVariables|SetbKeepSearching true)
  (LocalVariables|SetSafetyCounter 0)
  (while (LocalVariables|GetbKeepSearching)
    (Variables|Default|SetCurrentTurnIndex (+ (Variables|Default|GetCurrentTurnIndex) 1))
    (if (>= (Variables|Default|GetCurrentTurnIndex) (Utilities|Array|Length (Variables|Default|GetInitiativeOrder)))
      (Variables|Default|SetCurrentTurnIndex 0)
      (Variables|Default|SetCurrentRound (+ (Variables|Default|GetCurrentRound) 1))
      (Default|PostMessage (Variables|Default|GetTextManagerRef) (Utilities|Text|ToText(String) (Utilities|String|Append "ROUND: " (Utilities|String|ToString(Integer) (Variables|Default|GetCurrentRound)))) "NewEnumerator1"))
    (Variables|Default|SetCurrentCombatantID (Utilities|Array|Get(acopy) (Variables|Default|GetInitiativeOrder) (Variables|Default|GetCurrentTurnIndex)))
    (bind _isincapacitated (Default|IsCombatantIncapacitated (Variables|Default|GetCombatManagerRef) (Variables|Default|GetCurrentCombatantID)))
    (if _isincapacitated
      (LocalVariables|SetbKeepSearching true)
      (else
        (LocalVariables|SetbKeepSearching false)))
    (LocalVariables|SetSafetyCounter (+ (LocalVariables|GetSafetyCounter) 1))
    (if (>= (LocalVariables|GetSafetyCounter) (Utilities|Array|Length (Variables|Default|GetInitiativeOrder)))
      (LocalVariables|SetbKeepSearching false))))

(fn DispatchTurn
  (params (CombatantID :type Integer))
  (Default|TickConditions (Variables|Default|GetCombatManagerRef) CombatantID)
  (Variables|Default|SetCurrentCombatantID CombatantID)
  (bind _bisplayercontrolled (CallFunction|FindActiveCombatant))
  (if _bisplayercontrolled
    (CallFunction|StartPlayerTurn CombatantID)
    (else
      (CallFunction|StartEnemyTurn CombatantID))))

(fn StartPlayerTurn
  (params (CombatantID :type Integer))
  (bind _combatants (Variables|Default|GetCombatants))
  (bind (_combatant _bfound) (CallFunction|FindCombatantbyID _combatants CombatantID))
  (bind (_combatantid _combatantname _isplayercontrolled _sourcecharacter _sourcemonster _ismonster _gridposition _currenthp _maxhp _defenserating _strikenumber _initiative _actionsremaining _movementrange _attacksremaining _hasactedthisround _conditions _tilesmovedthisturn _characterid _moralestate _groupid _attackrange) (Utilities|Struct|BreakS_Combatant _combatant))
  (Variables|Default|SetCurrentCombatantID CombatantID)
  (Variables|Default|SetbPlayerTurnActive true)
  (Variables|/Game/Blueprints/Combat/BP_CombatManager.BP_CombatManager_C|SetbPlayerTurnActive (Variables|Default|GetCombatManagerRef) true)
  (Variables|/Game/Blueprints/Combat/BP_CombatManager.BP_CombatManager_C|SetCurrentCombatantID (Variables|Default|GetCombatManagerRef) CombatantID)
  (if _bfound
    (Default|PostMessage (Variables|Default|GetTextManagerRef) (Utilities|Text|ToText(String) (Utilities|String|Append _combatantname "'s turn - choose an action")) "NewEnumerator1")
    (for (_array_element _array_index) (Variables|Default|GetCombatants)
      (if (== (.CombatantID (Utilities|Struct|BreakS_Combatant _array_element)) (Variables|Default|GetCurrentCombatantID))
        (Utilities|Array|SetArrayElem (Variables|Default|GetCombatants) _array_index (Utilities|Struct|MakeS_Combatant _combatantid _combatantname _isplayercontrolled _sourcecharacter _sourcemonster _ismonster _gridposition _currenthp _maxhp _defenserating _strikenumber _initiative _actionsremaining _movementrange _attacksremaining false _conditions 0 _characterid _moralestate _groupid _attackrange))
        (bind _outcombatant (Default|FindCombatantbyID (Variables|Default|GetCombatManagerRef) CombatantID))
        (Utilities|Array|SetArrayElem (Variables|/Game/Blueprints/Combat/BP_CombatManager.BP_CombatManager_C|GetCombatants (Variables|Default|GetCombatManagerRef)) _array_index (Utilities|Struct|MakeS_Combatant (.CombatantID (Utilities|Struct|BreakS_Combatant _outcombatant)) (.CombatantName (Utilities|Struct|BreakS_Combatant _outcombatant)) (.IsPlayerControlled (Utilities|Struct|BreakS_Combatant _outcombatant)) (.SourceCharacter (Utilities|Struct|BreakS_Combatant _outcombatant)) (.SourceMonster (Utilities|Struct|BreakS_Combatant _outcombatant)) (.IsMonster (Utilities|Struct|BreakS_Combatant _outcombatant)) (.GridPosition (Utilities|Struct|BreakS_Combatant _outcombatant)) (.CurrentHP (Utilities|Struct|BreakS_Combatant _outcombatant)) (.MaxHP (Utilities|Struct|BreakS_Combatant _outcombatant)) (.DefenseRating (Utilities|Struct|BreakS_Combatant _outcombatant)) (.StrikeNumber (Utilities|Struct|BreakS_Combatant _outcombatant)) (.Initiative (Utilities|Struct|BreakS_Combatant _outcombatant)) (.ActionsRemaining (Utilities|Struct|BreakS_Combatant _outcombatant)) (.MovementRange (Utilities|Struct|BreakS_Combatant _outcombatant)) (.AttacksRemaining (Utilities|Struct|BreakS_Combatant _outcombatant)) false (.Conditions (Utilities|Struct|BreakS_Combatant _outcombatant)) 0 (.CharacterID (Utilities|Struct|BreakS_Combatant _outcombatant)) (.MoraleState (Utilities|Struct|BreakS_Combatant _outcombatant)) (.GroupID (Utilities|Struct|BreakS_Combatant _outcombatant)) (.AttackRange (Utilities|Struct|BreakS_Combatant _outcombatant))))))))

(fn StartEnemyTurn
  (params (CombatantID :type Integer))
  (bind _combatants (Variables|Default|GetCombatants))
  (bind (_combatant _bfound) (CallFunction|FindCombatantbyID _combatants CombatantID))
  (bind (_combatantid _combatantname _isplayercontrolled _sourcecharacter _sourcemonster _ismonster _gridposition _currenthp _maxhp _defenserating _strikenumber _initiative _actionsremaining _movementrange _attacksremaining _hasactedthisround _conditions _tilesmovedthisturn _characterid _moralestate _groupid _attackrange) (Utilities|Struct|BreakS_Combatant _combatant))
  (Variables|Default|SetCurrentCombatantID CombatantID)
  (Variables|Default|SetbPlayerTurnActive false)
  (Variables|/Game/Blueprints/Combat/BP_CombatManager.BP_CombatManager_C|SetCurrentCombatantID (Variables|Default|GetCombatManagerRef) CombatantID)
  (if _bfound
    (Default|PostMessage (Variables|Default|GetTextManagerRef) (Utilities|Text|ToText(String) (Utilities|String|Append _combatantname " attacks")) "NewEnumerator1")
    (Variables|/Game/Blueprints/Combat/BP_EnemyAI.BP_EnemyAI_C|SetCombatManagerRef (Variables|Default|GetEnemyAIRef) (Variables|Default|GetCombatManagerRef))
    (Variables|/Game/Blueprints/Combat/BP_EnemyAI.BP_EnemyAI_C|SetPartyMangerRef (Variables|Default|GetEnemyAIRef) (Variables|Default|GetPartyManagerRef))
    (Default|RunEnemyTurn (Variables|Default|GetEnemyAIRef) (Utilities|Struct|MakeS_Combatant _combatantid _combatantname _isplayercontrolled _sourcecharacter _sourcemonster _ismonster _gridposition _currenthp _maxhp _defenserating _strikenumber _initiative _actionsremaining _movementrange _attacksremaining false _conditions 0 _characterid _moralestate _groupid _attackrange))))

(fn EndPlayerTurn
  (if (Variables|Default|GetbPlayerTurnActive)
    (Variables|Default|SetbPlayerTurnActive false)
    (Variables|/Game/Blueprints/Combat/BP_CombatManager.BP_CombatManager_C|SetbPlayerTurnActive (Variables|Default|GetCombatManagerRef) false)
    (Variables|/Game/Blueprints/Combat/BP_CombatManager.BP_CombatManager_C|SetbMoveMode (Variables|Default|GetCombatManagerRef) false)
    (Variables|/Game/Blueprints/Combat/BP_CombatManager.BP_CombatManager_C|SetbSelectingTarget (Variables|Default|GetCombatManagerRef) false)
    (Default|ClearHighlights (Variables|Default|GetCombatGridRef))
    (CallFunction|OnActionComplete)))

(fn FindStartCombatant
  (Variables|Default|SetCurrentCombatantID (Utilities|Array|Get(acopy) (Variables|Default|GetInitiativeOrder) (Variables|Default|GetCurrentTurnIndex)))
  (if (.bFound (CallFunction|FindCombatantbyID (Variables|Default|GetCombatants) (Variables|Default|GetCurrentCombatantID)))
    (if (.IsPlayerControlled (Utilities|Struct|BreakS_Combatant (.Combatant (CallFunction|FindCombatantbyID (Variables|Default|GetCombatants) (Variables|Default|GetCurrentCombatantID)))))
      (CallFunction|StartPlayerTurn (Variables|Default|GetCurrentCombatantID))
      (else
        (CallFunction|StartEnemyTurn (Variables|Default|GetCurrentCombatantID))))))

(fn BuildInitiativeOrder
  (for (_array_element _array_index) (Variables|Default|GetCombatants)
    (bind _total (CallFunction|DiceRoll 1 10))
    (Utilities|Array|SetArrayElem (Variables|Default|GetCombatants) _array_index (Utilities|Struct|MakeS_Combatant (.CombatantID (Utilities|Struct|BreakS_Combatant _array_element)) (.CombatantName (Utilities|Struct|BreakS_Combatant _array_element)) (.IsPlayerControlled (Utilities|Struct|BreakS_Combatant _array_element)) (.SourceCharacter (Utilities|Struct|BreakS_Combatant _array_element)) (.SourceMonster (Utilities|Struct|BreakS_Combatant _array_element)) (.IsMonster (Utilities|Struct|BreakS_Combatant _array_element)) (.GridPosition (Utilities|Struct|BreakS_Combatant _array_element)) (.CurrentHP (Utilities|Struct|BreakS_Combatant _array_element)) (.MaxHP (Utilities|Struct|BreakS_Combatant _array_element)) (.DefenseRating (Utilities|Struct|BreakS_Combatant _array_element)) (.StrikeNumber (Utilities|Struct|BreakS_Combatant _array_element)) _total (.ActionsRemaining (Utilities|Struct|BreakS_Combatant _array_element)) (.MovementRange (Utilities|Struct|BreakS_Combatant _array_element)) (.AttacksRemaining (Utilities|Struct|BreakS_Combatant _array_element)) (.HasActedThisRound (Utilities|Struct|BreakS_Combatant _array_element)) (.Conditions (Utilities|Struct|BreakS_Combatant _array_element)) (.TilesMovedThisTurn (Utilities|Struct|BreakS_Combatant _array_element)) (.CharacterID (Utilities|Struct|BreakS_Combatant _array_element)) (.MoraleState (Utilities|Struct|BreakS_Combatant _array_element)) (.GroupID (Utilities|Struct|BreakS_Combatant _array_element)) (.AttackRange (Utilities|Struct|BreakS_Combatant _array_element)))))
  (CallFunction|SortInitiativeOrder))

(fn SortInitiativeOrder
  (Utilities|Array|Clear (Variables|Default|GetInitiativeOrder))
  (for _index (range 0 (- (Utilities|Array|Length (Variables|Default|GetCombatants)) 1))
    (LocalVariables|SetLowestInt 999)
    (LocalVariables|SetLowestID -1)
    (for _array_element (Variables|Default|GetCombatants)
      (if (and (not (Utilities|Array|ContainsItem (Variables|Default|GetInitiativeOrder) (.CombatantID (Utilities|Struct|BreakS_Combatant _array_element)))) (< (.Initiative (Utilities|Struct|BreakS_Combatant _array_element)) (LocalVariables|GetLowestInt)))
        (LocalVariables|SetLowestInt (.Initiative (Utilities|Struct|BreakS_Combatant _array_element)))
        (LocalVariables|SetLowestID (.CombatantID (Utilities|Struct|BreakS_Combatant _array_element)))))
    (if (!= (LocalVariables|GetLowestID) -1)
      (Utilities|Array|Add (Variables|Default|GetInitiativeOrder) (LocalVariables|GetLowestID)))))

(fn FindCombatantbyID
  (params (CombatantID :type Integer))
  (LocalVariables|SetbLocalFound false)
  (for (_array_element _array_index) (Variables|Default|GetCombatants)
    (if (== (.CombatantID (Utilities|Struct|BreakS_Combatant _array_element)) CombatantID)
      (LocalVariables|SetLocalOutCombatant _array_element)
      (LocalVariables|SetLocalOutIndex _array_index)
      (LocalVariables|SetbLocalFound true)))
  (return (LocalVariables|GetLocalOutCombatant) (LocalVariables|GetLocalOutIndex) (LocalVariables|GetbLocalFound)))