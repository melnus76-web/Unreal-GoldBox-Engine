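; Combat manager that runs turn-based, grid-based encounters between the party and a monster from DT_Monsters.
; StartCombat switches game state, generates the grid from the dungeon, places combatants on traversable tiles, rolls d10 initiative (lowest first), spawns markers and blends to the combat camera, locking explorer movement.
; Turns cycle through the initiative order, counting rounds.
; Player turns only prompt for an action; enemy turns post an attack message and immediately advance.
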(event EventBeginPlay
  ;[0.15 0.15 0.15 0.5] Temp
)

(event Collision|EventActorBeginOverlap
  (params (OtherActor :type Actor%20Object%20Reference)))

(event EventTick
  (params (DeltaSeconds :type Float%20%28single-precision%29)))

(fn ConstructionScript)

(fn StartCombat
  (params (MonsterGroupID :type Integer))
  (bind _gamemanagerref (Variables|Default|GetGameManagerRef))
  ;[0.15 0.15 0.15 0.5] Check for existing combat state
  (if (Variables|Default|GetbCombatActive)
    (Development|PrintString "StartCombat called but combat already active")
    (else
      ;[0.15 0.15 0.15 0.5] Change to Combat game state
      (Variables|Default|SetbCombatActive true)
      (Default|ChangeGameState (Variables|Default|GetGameManagerRef) "NewEnumerator3")
      (Default|PostMessage (Variables|Default|GetTextManagerRef) "Combat begins!" "NewEnumerator1")
      ;[0.15 0.15 0.15 0.5] Monster Lookup
      (bind _returnvalue (Utilities|GetDataTableRow "/Game/Blueprints/Data/DT_Monsters.DT_Monsters" (Utilities|String|StringToName (Utilities|String|ToString(Integer) MonsterGroupID)))
        (:then
          ;[0.15 0.15 0.15 0.5] Generate combat grid from player position
          (Default|GenerateGridfromDungeon (Variables|Default|GetCombatGridRef) (Variables|/Game/Blueprints/Core/BP_GameManager.BP_GameManager_C|GetCurrentPlayerTileX _gamemanagerref) (Variables|/Game/Blueprints/Core/BP_GameManager.BP_GameManager_C|GetCurrentPlayerTileY _gamemanagerref))
          (CallFunction|BuildCombatants _returnvalue)
          (CallFunction|BuildInitiativeOrder)
          (CallFunction|FindStartCombatant)
          (CallFunction|SpawnCombatantMarkers)
          (CallFunction|TransitiontoCombat))
        (:RowNotFound
          (Development|PrintString "Monster Not Found!!"))))))

(fn BuildInitiativeOrder
  (Utilities|Array|Clear (Variables|Default|GetInitiativeOrder))
  (for (_ _array_index) (Variables|Default|GetCombatants)
    (bind _total (CallFunction|DiceRoll 1 10))
    (Utilities|Array|SetArrayElem (Variables|Default|GetCombatants) _array_index (Utilities|Struct|MakeS_Combatant (.CombatantID (Utilities|Struct|BreakS_Combatant (Utilities|Array|Get(acopy) (Variables|Default|GetCombatants) _array_index))) (.CombatantName (Utilities|Struct|BreakS_Combatant (Utilities|Array|Get(acopy) (Variables|Default|GetCombatants) _array_index))) (.IsPlayerControlled (Utilities|Struct|BreakS_Combatant (Utilities|Array|Get(acopy) (Variables|Default|GetCombatants) _array_index))) (.SourceCharacter (Utilities|Struct|BreakS_Combatant (Utilities|Array|Get(acopy) (Variables|Default|GetCombatants) _array_index))) (.SourceMonster (Utilities|Struct|BreakS_Combatant (Utilities|Array|Get(acopy) (Variables|Default|GetCombatants) _array_index))) (.IsMonster (Utilities|Struct|BreakS_Combatant (Utilities|Array|Get(acopy) (Variables|Default|GetCombatants) _array_index))) (.GridPosition (Utilities|Struct|BreakS_Combatant (Utilities|Array|Get(acopy) (Variables|Default|GetCombatants) _array_index))) (.CurrentHP (Utilities|Struct|BreakS_Combatant (Utilities|Array|Get(acopy) (Variables|Default|GetCombatants) _array_index))) (.MaxHP (Utilities|Struct|BreakS_Combatant (Utilities|Array|Get(acopy) (Variables|Default|GetCombatants) _array_index))) (.AC (Utilities|Struct|BreakS_Combatant (Utilities|Array|Get(acopy) (Variables|Default|GetCombatants) _array_index))) (.THAC0 (Utilities|Struct|BreakS_Combatant (Utilities|Array|Get(acopy) (Variables|Default|GetCombatants) _array_index))) _total (.ActionsRemaining (Utilities|Struct|BreakS_Combatant (Utilities|Array|Get(acopy) (Variables|Default|GetCombatants) _array_index))) (.MovementRange (Utilities|Struct|BreakS_Combatant (Utilities|Array|Get(acopy) (Variables|Default|GetCombatants) _array_index))) (.AttacksRemaining (Utilities|Struct|BreakS_Combatant (Utilities|Array|Get(acopy) (Variables|Default|GetCombatants) _array_index))) (.HasActedThisRound (Utilities|Struct|BreakS_Combatant (Utilities|Array|Get(acopy) (Variables|Default|GetCombatants) _array_index))) (.Conditions (Utilities|Struct|BreakS_Combatant (Utilities|Array|Get(acopy) (Variables|Default|GetCombatants) _array_index))))))
  (CallFunction|SortInitiativeOrder))

(fn SortInitiativeOrder
  (Utilities|Array|Clear (Variables|Default|GetInitiativeOrder))
  ;[0.15 0.15 0.15 0.5] Outer Loop
  (for _index (range 0 (- (Utilities|Array|Length (Variables|Default|GetCombatants)) 1))
    (LocalVariables|SetLowestInit 999)
    (LocalVariables|SetLowestID -1)
    ;[0.15 0.15 0.15 0.5] Inner Loop
    (for _array_element (Variables|Default|GetCombatants)
      (if (and (not (Utilities|Array|ContainsItem (Variables|Default|GetInitiativeOrder) (.CombatantID (Utilities|Struct|BreakS_Combatant _array_element)))) (< (.Initiative (Utilities|Struct|BreakS_Combatant _array_element)) (LocalVariables|GetLowestInit)))
        (LocalVariables|SetLowestInit (.Initiative (Utilities|Struct|BreakS_Combatant _array_element)))
        (LocalVariables|SetLowestID (.CombatantID (Utilities|Struct|BreakS_Combatant _array_element)))))
    (if (!= (LocalVariables|GetLowestID) -1)
      (Utilities|Array|Add (Variables|Default|GetInitiativeOrder) (LocalVariables|GetLowestID)))))

(fn BuildCombatants
  (params (SourceMonster :type S%20Monster%20Structure))
  (bind (_currenthp _maxhp _ac _thac0 _condition _monsterid _monstername _hitdice _numattacks _damageperattack _movementrate) (Utilities|Struct|BreakS_Monster SourceMonster))
  ;[0.15 0.15 0.15 0.5] Monsters
  (bind (_foundx _foundy _bfound) (Default|FindNearestTraverrsableTile (Variables|Default|GetCombatGridRef) 14 8))
  (if _bfound
    (LocalVariables|SetMonsterSpawnPos (Math|Vector2D|MakeVector2D (Math|Conversions|ToFloat(Integer) _foundx) (Math|Conversions|ToFloat(Integer) _foundy)))
    (Default|SetOccupant (Variables|Default|GetCombatGridRef) _foundx _foundy 1)
    (else
      (LocalVariables|SetMonsterSpawnPos (Math|Vector2D|MakeVector2D 14.0 8.0))
      (Default|SetOccupant (Variables|Default|GetCombatGridRef) 14 8 1)))
  (Utilities|Array|Add (Variables|Default|GetCombatants) (Utilities|Struct|MakeS_Combatant 1 _monstername false "(CharacterName_2_6D849A044C63954D239677836D43CC06=\"\",Race_13_143D430A4900CC45B7E6E89F00C52BAB=NewEnumerator0,Class1_14_A7CFAE574CC4A293D58ACCA57149BCD4=NewEnumerator0,Class2_15_C474A67044B31C8FFD85E8B565EC27E6=NewEnumerator0,Alignment_16_210B85064898A886EAE2B99CAA976864=NewEnumerator0,Gender_12_A4BABCE741A71D222189E3A79900BE89=\"\",Strength_31_39829D1144593C09B82A2E952C1E15FC=0,StrengthExceptional_32_D260217D400A1E8402A03297D3F43C12=0,Intelligence_33_32B80A45429FBFD8FD4E28B61396B77B=0,Wisdom_34_6128C3A745371B2F60FA7D9E8A40B875=0,Dexterity_35_5441A5D6479A25488D769E9A67CBA618=0,Constitution_36_2B45005243924B3DF448219C7DE87E35=0,Charisma_37_8319D23F47B0C4ED99A87D8FF5A987F9=0,CurrentHP_45_96F669CE46972F15863BB68E8202E130=0,MaxHP_46_E784691048A496D20D0E2784D740327F=0,AC_47_DCD13A4F41ED5D34EEC93684FB870494=0,THAC0_48_7956888C4BB2FEE1585AB4A1FF0D5CA1=0,XP_49_1F3F3BB848BF010F331B5BA5BD897F25=0,Level_50_0B58E31041CBE5D682AE08AABD73487D=0,Level2_51_6E38D33A4D8D3490B43B92BFC7732B6E=0,Condition_54_1A2087B04B1D2902FA9A98A818BDF5AC=NewEnumerator0,SaveVsPoison_65_923F9C5841B3B820BCF57BAB18D616E0=0,SaveVsWands_66_2BE2CF884DFCCB039CB805BCE2767C06=0,SaveVsPetrification_67_AA122C344B82BFCA0FB383B0BC5B8183=0,SaveVsBreath_68_30B3AA814D0D992F8896F6BE00258307=0,SaveVsSpells_69_46ECE3EB4E2EB149038B15A5F01714A3=0,SpellSlotsCurrentL1_84_221C7DAF4054C6473AA967B92E76D016=0,SpellSlotsMaxL1_91_8D0C1AB04E5C51440E44EB88F679FE6B=0,SpellSlotsCurrentL2_85_1B66351641AC43E6359C659176EB4B16=0,SpellSlotsMaxL2_92_8629E5324BABA10B3B7B4D835B8F621A=0,SpellSlotsCurrentL3_86_14904A064BB223B6654595B540C76941=0,SpellSlotsMaxL3_93_7AF52DD443C32B48A56BEAA403E62143=0,SpellSlotsCurrentL4_87_9AF884164E4F2B707276D996CDA671F7=0,SpellSlotsMaxL4_94_888A1F914189EE5DE277569752428CF9=0,SpellSlotsCurrentL5_88_6F4FB69F443D2D55C4AA908EB4B2D903=0,SpellSlotsMaxL5_95_945250274E03434799ED3B8CB7927398=0,SpellSlotsCurrentL6_89_DDAF6DE041B59818CB7370A91883ABA4=0,SpellSlotsMaxL6_96_22AC1D4E4C998BF6799518B1B644EC81=0,SpellSlotsCurrentL7_90_C93745954074CDA83CFB6F8AB6243F89=0,SpellSlotsMaxL7_97_D99F40944CD1E8702F5AFE88526EEF3A=0,MemorisedSpellsL1_112_CE9FE51342F293F78B2EBE81A078A8AD=,MemorisedSpellsL2_113_BAE3ADDD4A71DCD5D8E22893D3D37495=,MemorisedSpellsL3_114_DBEC231D4083EC967F98E59E53C2D974=,MemorisedSpellsL4_152_E25B97CA4FC9D829D9EE3BB4F6AE12C7=,MemorisedSpellsL5_149_8C97B80042AE33BE16E3129AD8083CF3=,MemorisedSpellsL6_151_3D9DAE5048EFE549AEA27BBDA929EBCE=,MemorisedSpellsL7_150_FBFB108E4A141A1F951603AABD33CEAA=,EquipWeapon_144_B8F810D847CF7861E2774AAEFCA89877=0,EquipShield_143_C00391974C455725B65EFC92CB870354=0,EquipArmour_142_CAE4760B421063C628323B9F0AC943BE=0,EquipHelmet_141_7EF6093140C3DF4913899AAABE9F606F=0,EquipRing1_140_0BF5A11B44C53ADD610138A184B06A24=0,EquipRing2_139_B20847B84BD226D5D347898D4B977F5F=0,EquipCloak_138_D9D725CC4CCB3131B58B1F95E69D66C8=0,EquipMisc_137_F323CB92455F56709B252289A1C400D2=0,Inventory_136_17DDC40C4B7D9897A6D6EC8015459A09=,SkillPickPockets_163_DEB28EE64ACF08A5C878B7AA4B0B9D21=0,SkillOpenLocks_179_2742912F4FB796C9F7A923913E7D722A=0,SkillFindTraps_180_1E06DED945939CF03FCA4E86883BEA7A=0,SkillRemoveTraps_181_25A17079491F59E7085AF490F31DA966=0,SkillMoveSilently_182_729F0F9A4DDAE175F573878FA99BF92D=0,SkillHideInShadows_183_52A0C1534BB025731385D59AED552CE7=0,SkillHearNoise_184_0483B2754A16959E660120B4AED49EA7=0,SkillClimbWalls_185_BE4BAE0D4F81B5583A161B8B6D6F211A=0,SkillReadLanguages_186_A5CACD834F48C8AA7E12F0A8174F3EEA=0,Protrait_178_2F8879684520F64F7409F58E0D22FB0E=0,IsPlayerControlled_177_DD53BE0F41457ECB2F948685C020C902=False)" SourceMonster true (LocalVariables|GetMonsterSpawnPos) _currenthp _maxhp _ac _thac0 0 1 _movementrate _numattacks false "NewEnumerator0"))
  ;[0.15 0.15 0.15 0.5] Find Nearest Traversable tile
  ;;[0.15 0.15 0.15 0.5] Inner Loop
  (for (_array_element _array_index) (Default|GetPartyMembers (Variables|Default|GetPartyManagerRef))
    (bind _output_get (LocalVariables|SetPreferredY (+ 6 _array_index)))
    (bind (_foundx_2 _foundy_2 _bfound_2) (Default|FindNearestTraverrsableTile (Variables|Default|GetCombatGridRef) 1 _output_get))
    (if _bfound_2
      (LocalVariables|SetPartySpwanPos (Math|Vector2D|MakeVector2D (Math|Conversions|ToFloat(Integer) _foundx_2) (Math|Conversions|ToFloat(Integer) _foundy_2)))
      (Default|SetOccupant (Variables|Default|GetCombatGridRef) _foundx_2 _foundy_2 (+ _array_index 1000))
      (else
        (LocalVariables|SetPartySpwanPos (Math|Vector2D|MakeVector2D 1.0 (Math|Conversions|ToFloat(Integer) _output_get)))
        (Default|SetOccupant (Variables|Default|GetCombatGridRef) 1 _output_get (+ _array_index 1000))))
    (Utilities|Array|Add (Variables|Default|GetCombatants) (Utilities|Struct|MakeS_Combatant (+ _array_index 1000) (.CharacterName (Utilities|Struct|BreakS_Character _array_element)) true _array_element "(CurrentHP_10_E272B01549541D3F90E2F3A992DAA080=0,MaxHP_11_BA04E58647244E4A1FDB8C8C53AC7574=0,AC_12_E6A788C642C0949267B0EAB77604BD87=0,THAC0_14_FE9A813B4D97724A362ABE8B9815474C=0,Condition_15_E87EA1A943D4FD8B84D0DF8AAEA91F99=NewEnumerator0,MonsterID_20_8881546A460FB011C616689AD4D360C7=0,MonsterName_21_FC18DBB140C5B5B209A398A6C2F2FB2B=\"\",HitDice_30_14EB5399419ED41078146FA5487F01AF=0.000000,NumAttacks_31_3C3D73CD4DC3B285D4E88F8C507469D4=0,DamagePerAttack_33_BA17BA084D9CBA9D7386A58ED54513D9=,MovementRate_34_6581E3884505A9D36561C7BE1773A641=0,HasBreathWeapon_49_A449CBD74FB308D06163E9B10E71C528=False,HasLevelDrain_50_1934A63A45D1F2BCE4C2C3902770399B=False,HasPoison_51_F22A8774414C3CF0F4584880C151175A=False,HasPetrify_52_D91270E14A3DE417D3C16C997BB2BB55=False,IsSpellCaster_53_CE4B9BB3443C33A2410E3A988781C456=False,HasMagicResistance_54_1BE0F69B4B5896020D9E87A4EA1F5375=False,MagicResistance_48_C3617A1F4A78508239C74D9F0F9408DC=0,MoraleRating_79_3058D24B46894841304029991ADC485A=0,XPValue_78_22C561E44ADF28C34E5EE0AE5805A296=0,SpellList_62_891352464DA25F98FC008B9E1A507C66=,PortraitID_73_0AA973804163224E2D77448C1CAB8D89=0,IsUndead_72_BD2FA7D146DE75E7A27A9F9B52719380=False,IsGiantClass_76_9935D5BE42CD299267BD998A8CACA931=False,IsDemonic_77_42EECCF24656683513EAEBAE3193422B=False)" false (LocalVariables|GetPartySpwanPos) (.CurrentHP (Utilities|Struct|BreakS_Character _array_element)) (.MaxHP (Utilities|Struct|BreakS_Character _array_element)) (.AC (Utilities|Struct|BreakS_Character _array_element)) (.THAC0 (Utilities|Struct|BreakS_Character _array_element)) 0 1 12 1 false "NewEnumerator0"))))

(fn SpawnCombatantMarkers
  ;[0.15 0.15 0.15 0.5] Clear existing markers
  (Utilities|Array|Clear (Variables|Default|GetSpawnedMarkers))
  ;[0.15 0.15 0.15 0.5] Loop through combatants
  (for _array_element (Variables|Default|GetCombatants)
    ;[0.15 0.15 0.15 0.5] Spawn Marker
    (bind _returnvalue (Game|SpawnActorfromClass "/Game/Blueprints/Combat/BP_CombatantMarker.BP_CombatantMarker_C" (Math|Transform|MakeTransform (Math|Vector|MakeVector (.x (Default|TiletoWorld (Variables|Default|GetCombatGridRef) (Math|Float|Truncate (.X (Math|Vector2D|BreakVector2D (.GridPosition (Utilities|Struct|BreakS_Combatant _array_element))))) (Math|Float|Truncate (.Y (Math|Vector2D|BreakVector2D (.GridPosition (Utilities|Struct|BreakS_Combatant _array_element))))))) (.y (Default|TiletoWorld (Variables|Default|GetCombatGridRef) (Math|Float|Truncate (.X (Math|Vector2D|BreakVector2D (.GridPosition (Utilities|Struct|BreakS_Combatant _array_element))))) (Math|Float|Truncate (.Y (Math|Vector2D|BreakVector2D (.GridPosition (Utilities|Struct|BreakS_Combatant _array_element))))))) 5e+01) "0, 0, 0" "1.000000,1.000000,1.000000") "Undefined" "MultiplyWithRoot" 0 0))
    ;[0.15 0.15 0.15 0.5] Initialise marker
    (Default|Initialise _returnvalue (.CombatantName (Utilities|Struct|BreakS_Combatant _array_element)) (.IsMonster (Utilities|Struct|BreakS_Combatant _array_element)))
    ;[0.15 0.15 0.15 0.5] Store marker ref
    (Utilities|Array|Add (Variables|Default|GetSpawnedMarkers) _returnvalue)))

(fn TransitiontoCombat
  ;[0.15 0.15 0.15 0.5] Switch Camera
  (Game|Player|SetViewTargetwithBlend (Game|GetPlayerController 0) (Variables|Default|GetCombatCameraRef) 0.0 "VTBlend_EaseInOut" 2.0 false)
  ;[0.15 0.15 0.15 0.5] Lock Player Movement
  (bind _asbp_explorer_pawn (Utilities|Casting|CastToBP_ExplorerPawn (Game|Player|GetPlayerPawn 0)))
  (Variables|/Game/Blueprints/Dungeon/BP_ExplorerPawn.BP_ExplorerPawn_C|SetCanMove _asbp_explorer_pawn false))

(fn StartPlayerTurn
  (params (CombatantID :type Integer))
  (Variables|Default|SetCurrentCombatantID CombatantID)
  (Variables|Default|SetbPlayerTurnActive true)
  ;[0.15 0.15 0.15 0.5] Find player combatant
  (for _array_element (Variables|Default|GetCombatants)
    (if (== (.CombatantID (Utilities|Struct|BreakS_Combatant _array_element)) CombatantID)
      ;[0.15 0.15 0.15 0.5] Post Message
      (Default|PostMessage (Variables|Default|GetTextManagerRef) (Utilities|Text|ToText(String) (Utilities|String|Append (.CombatantName (Utilities|Struct|BreakS_Combatant _array_element)) "'s turn - choose an action")) "NewEnumerator1"))))

(fn StartEnemyTurn
  (params (CombatantID :type Integer))
  (Variables|Default|SetCurrentCombatantID CombatantID)
  (Variables|Default|SetbPlayerTurnActive false)
  ;[0.15 0.15 0.15 0.5] Find Combatant
  (for _array_element (Variables|Default|GetCombatants)
    (if (== (.CombatantID (Utilities|Struct|BreakS_Combatant _array_element)) CombatantID)
      ;[0.15 0.15 0.15 0.5] Post Message
      (Default|PostMessage (Variables|Default|GetTextManagerRef) (Utilities|Text|ToText(String) (Utilities|String|Append (.CombatantName (Utilities|Struct|BreakS_Combatant _array_element)) " attacks!")) "NewEnumerator0")
      (CallFunction|OnActionComplete))))

(fn OnActionComplete
  ;[0.15 0.15 0.15 0.5] Set turn index
  (bind _output_get (Variables|Default|SetCurrentTurnIndex (+ (Variables|Default|GetCurrentTurnIndex) 1)))
  ;[0.15 0.15 0.15 0.5] Chcek if all combatants have acted
  (if (>= _output_get (Utilities|Array|Length (Variables|Default|GetInitiativeOrder)))
    ;[0.15 0.15 0.15 0.5] Increase Combat Round Number
    (Variables|Default|SetCurrentTurnIndex 0)
    (bind _output_get_2 (Variables|Default|SetCurrentRound (+ (Variables|Default|GetCurrentRound) 1)))
    ;[0.15 0.15 0.15 0.5] Post Message
    (Default|PostMessage (Variables|Default|GetTextManagerRef) (Utilities|Text|ToText(String) (Utilities|String|Append "Round " (Utilities|String|ToString(Integer) _output_get_2))) "NewEnumerator1"))
  ;[0.15 0.15 0.15 0.5] Find next combatant
  (Variables|Default|SetCurrentCombatantID (Utilities|Array|Get(acopy) (Variables|Default|GetInitiativeOrder) (Variables|Default|GetCurrentTurnIndex)))
  ;[0.15 0.15 0.15 0.5] Determin PLayer ormonster to act
  (for _array_element (Variables|Default|GetCombatants)
    (if (== (.CombatantID (Utilities|Struct|BreakS_Combatant _array_element)) (Utilities|Array|Get(acopy) (Variables|Default|GetInitiativeOrder) (Variables|Default|GetCurrentTurnIndex)))
      (if (.IsPlayerControlled (Utilities|Struct|BreakS_Combatant _array_element))
        (CallFunction|StartPlayerTurn (.CombatantID (Utilities|Struct|BreakS_Combatant _array_element)))
        (else
          (CallFunction|StartEnemyTurn (.CombatantID (Utilities|Struct|BreakS_Combatant _array_element))))))))

(fn FindStartCombatant
  (for _array_element (Variables|Default|GetCombatants)
    (if (not (LocalVariables|GetbFound))
      (if (== (Utilities|Array|Get(acopy) (Variables|Default|GetInitiativeOrder)) (.CombatantID (Utilities|Struct|BreakS_Combatant _array_element)))
        (LocalVariables|SetbFound true)
        (if (.IsPlayerControlled (Utilities|Struct|BreakS_Combatant _array_element))
          (CallFunction|StartPlayerTurn (.CombatantID (Utilities|Struct|BreakS_Combatant _array_element)))
          (else
            (CallFunction|StartEnemyTurn (.CombatantID (Utilities|Struct|BreakS_Combatant _array_element))))))))
  (return))