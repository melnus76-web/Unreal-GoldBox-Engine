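; Blueprint function library of shared RPG rules helpers for dice rolls and UI colour coding.
; HP helpers compute a clamped, zero-safe health fraction and map it to a bar colour by thresholds.
; Lookup functions map character conditions and message log types to colours, with several severe conditions sharing one dark red.
; Dice helpers sum random rolls, optionally add a modifier, or roll a percentile.
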(fn GetHPFraction
  (params (CurrentHP :type Integer) (MaxHP :type Integer))
  (if (> MaxHP 0)
    (return (Math|Float|Clamp(Float) (/ (Math|Conversions|ToFloat(Integer) CurrentHP) (Math|Conversions|ToFloat(Integer) MaxHP))))
    (else
      (return 0.0))))

(fn GetHPBarColor
  (params (HPFraction :type Float%20%28double-precision%29))
  (if (> HPFraction 0.6)
    (return (Utilities|Struct|MakeLinearColor 0.2 0.8 0.2 1.0))
    (elif (> HPFraction 0.3)
      (return (Utilities|Struct|MakeLinearColor 0.9 0.75 0.1 1.0))
      (elif (> HPFraction 0.0)
        (return (Utilities|Struct|MakeLinearColor 0.9 0.35 0.1 1.0))
        (else
          (return (Utilities|Struct|MakeLinearColor 0.3 0.3 0.3 1.0)))))))

(fn GetConditionColor
  (params (Condition :type E_Condition%20Enum :default "NewEnumerator0"))
  (switch Utilities|FlowControl|Switch|SwitchonE_Condition Condition
    (:NewEnumerator0
      (return (Utilities|Struct|MakeLinearColor 0.0 0.0 0.0 0.0)))
    (:NewEnumerator1
      (return (Utilities|Struct|MakeLinearColor 0.7 0.4 0.9 1.0)))
    (:NewEnumerator2
      (return (Utilities|Struct|MakeLinearColor 0.7 0.4 0.9 1.0)))
    (:NewEnumerator3
      (return (Utilities|Struct|MakeLinearColor 0.6 0.9 0.1 1.0)))
    (:NewEnumerator4
      (return (Utilities|Struct|MakeLinearColor 0.8 0.6 0.1 1.0)))
    (:NewEnumerator5
      (return (Utilities|Struct|MakeLinearColor 0.1 0.9 0.9 1.0)))
    (:NewEnumerator6
      (return (Utilities|Struct|MakeLinearColor 0.5 0.5 0.7 1.0)))
    (:NewEnumerator7
      (return (Utilities|Struct|MakeLinearColor 0.4 0.1 0.1 1.0)))
    (:NewEnumerator8
      (return (Utilities|Struct|MakeLinearColor 0.4 0.1 0.1 1.0)))
    (:NewEnumerator9
      (return (Utilities|Struct|MakeLinearColor 0.4 0.1 0.1 1.0)))
    (:NewEnumerator10
      (return (Utilities|Struct|MakeLinearColor 0.4 0.1 0.1 1.0)))
    (:NewEnumerator11
      (return (Utilities|Struct|MakeLinearColor 0.4 0.1 0.1 1.0)))))

(fn GetMessageColor
  (params (MessageType :type E_MessageType%20Enum :default "NewEnumerator0"))
  (switch Utilities|FlowControl|Switch|SwitchonE_MessageType MessageType
    (:NewEnumerator0
      (return (Utilities|Struct|MakeLinearColor 0.78 0.72 0.48 1.0)))
    (:NewEnumerator1
      (return (Utilities|Struct|MakeLinearColor 0.9 0.4 0.3 1.0)))
    (:NewEnumerator2
      (return (Utilities|Struct|MakeLinearColor 0.3 0.7 0.3 1.0)))
    (:NewEnumerator3
      (return (Utilities|Struct|MakeLinearColor 0.5 0.8 0.9 1.0)))
    (:NewEnumerator4
      (return (Utilities|Struct|MakeLinearColor 0.7 0.5 0.9 1.0)))))

(fn DiceRoll
  (params (NumDice :type Integer) (DiceType :type Integer))
  (for _index (range 0 (- NumDice 1))
    (bind _output_get (LocalVariables|SetRunningTotal (+ (LocalVariables|GetRunningTotal) (Math|Random|RandomIntegerinRange 1 DiceType)))))
  (return _output_get))

(fn DiceRollwithModifier
  (params (NumDice :type Integer) (DieType :type Integer) (Modifier :type Integer))
  (bind _total (CallFunction|DiceRoll NumDice DieType))
  (return (+ _total Modifier)))

(fn PercentileRoll
  (return (Math|Random|RandomIntegerinRange 1 100)))