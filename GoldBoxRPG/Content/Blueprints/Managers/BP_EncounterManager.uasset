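; Encounter manager that runs data-driven, choice-based encounters for the explorer pawn.
; StartEncounter loads a DT_Encounters row by ID, changes game state, posts intro text and shows the portrait and choices on the encounter screen.
; ResolveChoice branches on outcome type: Combat hands a monster group to the game instance's CombatManager, while Reward, Flee and Text Only post a message, restore game state and movement, and close the screen.
; GrantReward is an empty stub.
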(event EventBeginPlay)

(event Collision|EventActorBeginOverlap
  (params (OtherActor :type Actor%20Object%20Reference)))

(event EventTick
  (params (DeltaSeconds :type Float%20%28single-precision%29)))

(fn ConstructionScript)

(fn StartEncounter
  (params (EncounterID :type Integer))
  (bind _encounterscreenref (Variables|Default|GetEncounterScreenRef))
  (bind _output_get (Variables|Default|SetCurrentEncounterID EncounterID))
  (bind _returnvalue (Utilities|GetDataTableRow "/Game/Data/DataTables/DT_Encounters.DT_Encounters" (Utilities|String|StringToName (Utilities|String|ToString(Integer) _output_get)))
    (:then
      (if true
        (bind _output_get_2 (Variables|Default|SetCurrentEncounter _returnvalue))
        (Default|ShowPortrait (Variables|Default|GetEncounterScreenRef) (.PortraitID (Utilities|Struct|BreakS_Encounter _output_get_2)))
        (Default|ChangeGameState (Variables|Default|GetGameManagerRef) "NewEnumerator2")
        (Default|PostMessage (Variables|Default|GetTextManagerRef) (.IntroText (Utilities|Struct|BreakS_Encounter _output_get_2)) "NewEnumerator4")
        (Default|SetEncounterData (Variables|Default|GetEncounterScreenRef) (.IntroText (Utilities|Struct|BreakS_Encounter _output_get_2)) (.Choices (Utilities|Struct|BreakS_Encounter _output_get_2)))
        (Variables|/Game/Blueprints/UI/WBP_EncounterScreen.WBP_EncounterScreen_C|SetEncounterManagerRef _encounterscreenref 0)
        (UserInterface|Viewport|AddtoViewport _encounterscreenref 1)
        (else
          (Development|PrintString (Utilities|String|Append "Encounter Not Found: " (Utilities|String|ToString(Integer) _output_get))))))))

(fn ResolveChoice
  (params (ChoiceIndex :type Integer))
  (bind _currentencounter (Variables|Default|GetCurrentEncounter))
  (bind _choices (Utilities|Struct|BreakS_Encounter _currentencounter))
  (bind _output (Utilities|Array|Get(acopy) _choices ChoiceIndex))
  (bind (_choicelabel _outcometype _outcomepayload) (Utilities|Struct|BreakS_EncounterChoice _output))
  (bind _returnvalue (Utilities|Text|ToText(String) _outcomepayload))
  (switch Utilities|FlowControl|Switch|SwitchonE_OutcomeType _outcometype
    (:NewEnumerator0
      (CallFunction|TriggerCombatfromEncounter (Math|Conversions|ToInteger(Byte) _outcomepayload))
      (Widget|RemovefromParent (Variables|Default|GetEncounterScreenRef)))
    (:NewEnumerator1
      (CallFunction|GrantReward 0 (Math|Conversions|ToInteger(Byte) _outcomepayload))
      (Default|PostMessage (Variables|Default|GetTextManagerRef) "Reward Granted" "NewEnumerator4")
      (Default|ChangeGameState (Variables|Default|GetGameManagerRef) "NewEnumerator1" :!label _label)
      (Default|HidePortrait (Variables|Default|GetEncounterScreenRef))
      (Widget|RemovefromParent (Variables|Default|GetEncounterScreenRef))
      (bind _asbp_explorer_pawn (Utilities|Casting|CastToBP_ExplorerPawn (Game|Player|GetPlayerPawn 0)))
      (Variables|/Game/Blueprints/Dungeon/BP_ExplorerPawn.BP_ExplorerPawn_C|SetCanMove _asbp_explorer_pawn true))
    (:NewEnumerator2
      (Default|PostMessage (Variables|Default|GetTextManagerRef) _returnvalue "NewEnumerator4")
      (bind _asbp_explorer_pawn_2 (Utilities|Casting|CastToBP_ExplorerPawn (Game|Player|GetPlayerPawn 0)))
      (Variables|/Game/Blueprints/Dungeon/BP_ExplorerPawn.BP_ExplorerPawn_C|SetCanMove _asbp_explorer_pawn_2 false)
      (goto _label))
    (:NewEnumerator3
      (Default|PostMessage (Variables|Default|GetTextManagerRef) _returnvalue "NewEnumerator4")
      (goto _label))))

(fn TriggerCombatfromEncounter
  (params (MonsterGroupID :type Integer))
  (bind _asbp_game_manager (Utilities|Casting|CastToBP_GameManager (Game|GetGameInstance)))
  (Default|StartCombat (Variables|/Game/Blueprints/Core/BP_GameManager.BP_GameManager_C|GetCombatManagerRef _asbp_game_manager) MonsterGroupID))

(fn GrantReward
  (params (ItemID :type Integer) (XPAmount :type Integer)))