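; BP_EventManager fires data-driven events attached to map tiles, such as messages and encounters.
; EvaluateTriggers matches a tile's EventTriggerID against DT_TriggerEvents, passing active On Enter Tile rows without an "Encounter_<ID>" story flag to ExecuteTrigger.
; ExecuteTrigger posts messages through TextManagerRef or starts encounters through the GameManager's EncounterManager, setting that flag to prevent repeats.
; Combat, level transition, story flag and loot actions are unimplemented stubs.
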(event EventBeginPlay)

(event Collision|EventActorBeginOverlap
  (params (OtherActor :type Actor%20Object%20Reference)))

(event EventTick
  (params (DeltaSeconds :type Float%20%28single-precision%29)))

(fn ConstructionScript)

(fn EvaluateTriggers
  (params (TileX :type Integer) (TileY :type Integer) (TriggerType :type E_TriggerType%20Enum :default "NewEnumerator0"))
  (bind _mapmanagerref (Variables|Default|GetMapManagerRef))
  (bind _tile (Default|GetTile _mapmanagerref TileX TileY))
  (bind _eventtriggerid (Utilities|Struct|BreakS_DungeonTile _tile))
  (if (> _eventtriggerid 0)
    (bind _outrownames (DataTable|GetDataTableRowNames "/Game/Data/DataTables/DT_TriggerEvents.DT_TriggerEvents"))
    (for _array_element _outrownames
      (bind _returnvalue (Utilities|GetDataTableRow "/Game/Data/DataTables/DT_TriggerEvents.DT_TriggerEvents" _array_element)
        (:then
          (if (== (.triggerid _returnvalue) _eventtriggerid)
            (bind _asbp_game_manager (Utilities|Casting|CastToBP_GameManager (Game|GetGameInstance)))
            (bind _result (Default|CheckStoryFlag _asbp_game_manager (Utilities|String|Append "Encounter_" (Utilities|String|ToString(Integer) (.triggerid _returnvalue)))))
            (if (not _result)
              (switch Utilities|FlowControl|Switch|SwitchonE_TriggerType (.triggertype _returnvalue)
                (:NewEnumerator0
                  (if (.isactive _returnvalue)
                    (CallFunction|ExecuteTrigger (Utilities|Struct|MakeS_TriggerEvent (.triggerid _returnvalue) (.triggertype _returnvalue) (.actiontype _returnvalue) (.messagetext _returnvalue) (.encounterid _returnvalue) (.targetlevelid _returnvalue) (.storyflagname _returnvalue) (.storyflagvalue _returnvalue) (.oneshot _returnvalue) (.isactive _returnvalue)))))))))))))

(fn ExecuteTrigger
  (params (TriggerEvent :type S%20Trigger%20Event%20Structure))
  (bind (_triggerid _triggertype _actiontype _messagetext _encounterid) (Utilities|Struct|BreakS_TriggerEvent TriggerEvent))
  (switch Utilities|FlowControl|Switch|SwitchonE_TriggerActionType _actiontype
    (:NewEnumerator0
      (Default|PostMessage (Variables|Default|GetTextManagerRef) (Utilities|Text|ToText(String) _messagetext) "NewEnumerator0")
      (Development|PrintString _messagetext))
    (:NewEnumerator1
      (bind _asbp_game_manager (Utilities|Casting|CastToBP_GameManager (Game|GetGameInstance)))
      (Default|StartEncounter (Variables|/Game/Blueprints/Core/BP_GameManager.BP_GameManager_C|GetEncounterManagerRef _asbp_game_manager) _encounterid)
      (bind _asbp_game_manager_2 (Utilities|Casting|CastToBP_GameManager (Game|GetGameInstance)))
      (Default|SetStoryFlag _asbp_game_manager_2 (Utilities|String|Append "Encounter_" (Utilities|String|ToString(Integer) _triggerid)) true))
    (:NewEnumerator2
      (Development|PrintString "Not implemented yet" :!label _label))
    (:NewEnumerator3
      (goto _label))
    (:NewEnumerator4
      (goto _label))
    (:NewEnumerator5
      (goto _label))))