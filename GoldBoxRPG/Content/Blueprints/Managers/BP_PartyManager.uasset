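; BP_PartyManager holds the RPG party as an array of SCharacter structs and loads it from the CharacterRoster save on BeginPlay.
; Functions add members from saves or test DataTable rows, query living members, and rebuild structs to update XP, HP or death.
; Most changes to loading, HP and death fire OnPartyUpdated.
; Saving appends only the last member to an existing roster; AwardXPToParty is a print stub.
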(event EventBeginPlay
  (CallFunction|LoadSavedParty))

(event Collision|EventActorBeginOverlap
  (params (OtherActor :type Actor%20Object%20Reference)))

(event EventTick
  (params (DeltaSeconds :type Float%20%28single-precision%29)))

(fn ConstructionScript)

(fn AddCharacter
  (params (NewCharacter :type S%20Character%20Structure))
  (bind (_charactername _race _class1 _class2 _morality _gender _might _acuity _resolve _reflex _vigor _presence _currenthp _maxhp _defenserating _strikenumber _xp _level _level2 _condition _fortitudesave _reflexsave _resolvesave _spellslotscurrentl1 _spellslotsmaxl1 _spellslotscurrentl2 _spellslotsmaxl2 _spellslotscurrentl3 _spellslotsmaxl3 _spellslotscurrentl4 _spellslotsmaxl4 _spellslotscurrentl5 _spellslotsmaxl5 _spellslotscurrentl6 _spellslotsmaxl6 _spellslotscurrentl7 _spellslotsmaxl7 _memorisedspellsl1 _memorisedspellsl2 _memorisedspellsl3 _memorisedspellsl4 _memorisedspellsl5 _memorisedspellsl6 _memorisedspellsl7 _equipweapon _equipshield _equiparmour _equiphelmet _equipring1 _equipring2 _equipcloak _equipmisc _inventory _skillpickpockets _skillopenlocks _skillfindtraps _skillremovetraps _skillmovesilently _skillhideinshadows _skillhearnoise _skillclimbwalls _skillreadlanguages _protrait _isplayercontrolled) (Utilities|Struct|BreakS_Character NewCharacter))
  (Utilities|Array|Add (Variables|Default|GetPartyMembers) (Utilities|Struct|MakeS_Character _charactername _race _class1 _class2 _morality _gender _might _acuity _resolve _reflex _vigor _presence _currenthp _maxhp _defenserating _strikenumber _xp _level _level2 _condition _fortitudesave _reflexsave _resolvesave _spellslotscurrentl1 _spellslotsmaxl1 _spellslotscurrentl2 _spellslotsmaxl2 _spellslotscurrentl3 _spellslotsmaxl3 _spellslotscurrentl4 _spellslotsmaxl4 _spellslotscurrentl5 _spellslotsmaxl5 _spellslotscurrentl6 _spellslotsmaxl6 _spellslotscurrentl7 _spellslotsmaxl7 _memorisedspellsl1 _memorisedspellsl2 _memorisedspellsl3 _memorisedspellsl4 _memorisedspellsl5 _memorisedspellsl6 _memorisedspellsl7 _equipweapon _equipshield _equiparmour _equiphelmet _equipring1 _equipring2 _equipcloak _equipmisc _inventory _skillpickpockets _skillopenlocks _skillfindtraps _skillremovetraps _skillmovesilently _skillhideinshadows _skillhearnoise _skillclimbwalls _skillreadlanguages _protrait _isplayercontrolled (Utilities|Array|Length (Variables|Default|GetPartyMembers)))))

(fn GetLivingMembers
  (for _array_element (Variables|Default|GetPartyMembers)
    (LocalVariables|SetPartyMembersArrayElement _array_element)
    (if (not (Utilities|Array|ContainsItem (.Condition (Utilities|Struct|BreakS_Character (LocalVariables|GetPartyMembersArrayElement))) "NewEnumerator10"))
      (Utilities|Array|Add (LocalVariables|GetTempLiving) (LocalVariables|GetPartyMembersArrayElement))))
  (return (LocalVariables|GetTempLiving)))

(fn IsPartyWiped
  (return (== (Utilities|Array|Length (CallFunction|GetLivingMembers)) 0)))

(fn GetActiveSpeaker
  (return (Utilities|Array|Get(acopy) (CallFunction|GetLivingMembers))))

(fn ReorderParty
  (params (IndexA :type Integer) (IndexB :type Integer))
  (bind _partymembers (Variables|Default|GetPartyMembers))
  (Utilities|Array|SetArrayElem _partymembers IndexA (Utilities|Array|Get(acopy) _partymembers IndexB))
  (Utilities|Array|SetArrayElem _partymembers IndexB (Utilities|Array|Get(acopy) _partymembers IndexA)))

(fn AwardXPtoParty
  (params (Amount :type Integer))
  (Development|PrintString "AwardXPToParty called"))

(fn InitialiseTestParty
  (bind _returnvalue (Utilities|GetDataTableRow "/Game/Data/DataTables/DT_TestParty.DT_TestParty" (Utilities|String|StringToName (Utilities|String|MakeLiteralString "Fighter")))
    (:then
      (CallFunction|AddCharacter _returnvalue)
      (bind _returnvalue_2 (Utilities|GetDataTableRow "/Game/Data/DataTables/DT_TestParty.DT_TestParty" (Utilities|String|StringToName (Utilities|String|MakeLiteralString "Cleric")))
        (:then
          (CallFunction|AddCharacter _returnvalue_2)
          (bind _returnvalue_3 (Utilities|GetDataTableRow "/Game/Data/DataTables/DT_TestParty.DT_TestParty" (Utilities|String|StringToName (Utilities|String|MakeLiteralString "MagicUser")))
            (:then
              (CallFunction|AddCharacter _returnvalue_3)
              (bind _returnvalue_4 (Utilities|GetDataTableRow "/Game/Data/DataTables/DT_TestParty.DT_TestParty" (Utilities|String|StringToName (Utilities|String|MakeLiteralString "Thief")))
                (:then
                  (CallFunction|AddCharacter _returnvalue_4)
                  (Default|CallOnPartyUpdated))))))))))

(fn AddXPtoCharacter
  (params (CharacterID :type Integer) (XPAmount :type Integer))
  (for (_array_element _array_index) (Variables|Default|GetPartyMembers)
    (if (== (.CharacterID (Utilities|Struct|BreakS_Character _array_element)) CharacterID)
      (Utilities|Array|SetArrayElem (Variables|Default|GetPartyMembers) _array_index (Utilities|Struct|MakeS_Character (.CharacterName (Utilities|Struct|BreakS_Character _array_element)) (.Race (Utilities|Struct|BreakS_Character _array_element)) (.Class1 (Utilities|Struct|BreakS_Character _array_element)) (.Class2 (Utilities|Struct|BreakS_Character _array_element)) (.Morality (Utilities|Struct|BreakS_Character _array_element)) (.Gender (Utilities|Struct|BreakS_Character _array_element)) (.Might (Utilities|Struct|BreakS_Character _array_element)) (.Acuity (Utilities|Struct|BreakS_Character _array_element)) (.Resolve (Utilities|Struct|BreakS_Character _array_element)) (.Reflex (Utilities|Struct|BreakS_Character _array_element)) (.Vigor (Utilities|Struct|BreakS_Character _array_element)) (.Presence (Utilities|Struct|BreakS_Character _array_element)) (.CurrentHP (Utilities|Struct|BreakS_Character _array_element)) (.MaxHP (Utilities|Struct|BreakS_Character _array_element)) (.DefenseRating (Utilities|Struct|BreakS_Character _array_element)) (.StrikeNumber (Utilities|Struct|BreakS_Character _array_element)) (+ (.XP (Utilities|Struct|BreakS_Character _array_element)) XPAmount) (.Level (Utilities|Struct|BreakS_Character _array_element)) (.Level2 (Utilities|Struct|BreakS_Character _array_element)) (.Condition (Utilities|Struct|BreakS_Character _array_element)) (.FortitudeSave (Utilities|Struct|BreakS_Character _array_element)) (.ReflexSave (Utilities|Struct|BreakS_Character _array_element)) (.ResolveSave (Utilities|Struct|BreakS_Character _array_element)) (.SpellSlotsCurrentL1 (Utilities|Struct|BreakS_Character _array_element)) (.SpellSlotsMaxL1 (Utilities|Struct|BreakS_Character _array_element)) (.SpellSlotsCurrentL2 (Utilities|Struct|BreakS_Character _array_element)) (.SpellSlotsMaxL2 (Utilities|Struct|BreakS_Character _array_element)) (.SpellSlotsCurrentL3 (Utilities|Struct|BreakS_Character _array_element)) (.SpellSlotsMaxL3 (Utilities|Struct|BreakS_Character _array_element)) (.SpellSlotsCurrentL4 (Utilities|Struct|BreakS_Character _array_element)) (.SpellSlotsMaxL4 (Utilities|Struct|BreakS_Character _array_element)) (.SpellSlotsCurrentL5 (Utilities|Struct|BreakS_Character _array_element)) (.SpellSlotsMaxL5 (Utilities|Struct|BreakS_Character _array_element)) (.SpellSlotsCurrentL6 (Utilities|Struct|BreakS_Character _array_element)) (.SpellSlotsMaxL6 (Utilities|Struct|BreakS_Character _array_element)) (.SpellSlotsCurrentL7 (Utilities|Struct|BreakS_Character _array_element)) (.SpellSlotsMaxL7 (Utilities|Struct|BreakS_Character _array_element)) (.MemorisedSpellsL1 (Utilities|Struct|BreakS_Character _array_element)) (.MemorisedSpellsL2 (Utilities|Struct|BreakS_Character _array_element)) (.MemorisedSpellsL3 (Utilities|Struct|BreakS_Character _array_element)) (.MemorisedSpellsL4 (Utilities|Struct|BreakS_Character _array_element)) (.MemorisedSpellsL5 (Utilities|Struct|BreakS_Character _array_element)) (.MemorisedSpellsL6 (Utilities|Struct|BreakS_Character _array_element)) (.MemorisedSpellsL7 (Utilities|Struct|BreakS_Character _array_element)) (.EquipWeapon (Utilities|Struct|BreakS_Character _array_element)) (.EquipShield (Utilities|Struct|BreakS_Character _array_element)) (.EquipArmour (Utilities|Struct|BreakS_Character _array_element)) (.EquipHelmet (Utilities|Struct|BreakS_Character _array_element)) (.EquipRing1 (Utilities|Struct|BreakS_Character _array_element)) (.EquipRing2 (Utilities|Struct|BreakS_Character _array_element)) (.EquipCloak (Utilities|Struct|BreakS_Character _array_element)) (.EquipMisc (Utilities|Struct|BreakS_Character _array_element)) (.Inventory (Utilities|Struct|BreakS_Character _array_element)) (.SkillPickPockets (Utilities|Struct|BreakS_Character _array_element)) (.SkillOpenLocks (Utilities|Struct|BreakS_Character _array_element)) (.SkillFindTraps (Utilities|Struct|BreakS_Character _array_element)) (.SkillRemoveTraps (Utilities|Struct|BreakS_Character _array_element)) (.SkillMoveSilently (Utilities|Struct|BreakS_Character _array_element)) (.SkillHideInShadows (Utilities|Struct|BreakS_Character _array_element)) (.SkillHearNoise (Utilities|Struct|BreakS_Character _array_element)) (.SkillClimbWalls (Utilities|Struct|BreakS_Character _array_element)) (.SkillReadLanguages (Utilities|Struct|BreakS_Character _array_element)) (.Protrait (Utilities|Struct|BreakS_Character _array_element)) (.IsPlayerControlled (Utilities|Struct|BreakS_Character _array_element)) (.CharacterID (Utilities|Struct|BreakS_Character _array_element)))))))

(fn ApplyDeathtoCharacter
  (params (CharacterID :type Integer))
  ;[0.15 0.15 0.15 0.5] Comment
  (LocalVariables|SetLocalCharacterID CharacterID)
  (for (_array_element _array_index) (Variables|Default|GetPartyMembers)
    (if (== (LocalVariables|GetLocalCharacterID) (.CharacterID (Utilities|Struct|BreakS_Character _array_element)))
      (bind _output_get (LocalVariables|SetUpdatedConditions (.Condition (Utilities|Struct|BreakS_Character _array_element))))
      (Utilities|Array|Add _output_get "NewEnumerator10")
      (Utilities|Array|SetArrayElem (Variables|Default|GetPartyMembers) _array_index (Utilities|Struct|MakeS_Character (.CharacterName (Utilities|Struct|BreakS_Character _array_element)) (.Race (Utilities|Struct|BreakS_Character _array_element)) (.Class1 (Utilities|Struct|BreakS_Character _array_element)) (.Class2 (Utilities|Struct|BreakS_Character _array_element)) (.Morality (Utilities|Struct|BreakS_Character _array_element)) (.Gender (Utilities|Struct|BreakS_Character _array_element)) (.Might (Utilities|Struct|BreakS_Character _array_element)) (.Acuity (Utilities|Struct|BreakS_Character _array_element)) (.Resolve (Utilities|Struct|BreakS_Character _array_element)) (.Reflex (Utilities|Struct|BreakS_Character _array_element)) (.Vigor (Utilities|Struct|BreakS_Character _array_element)) (.Presence (Utilities|Struct|BreakS_Character _array_element)) 0 (.MaxHP (Utilities|Struct|BreakS_Character _array_element)) (.DefenseRating (Utilities|Struct|BreakS_Character _array_element)) (.StrikeNumber (Utilities|Struct|BreakS_Character _array_element)) (.XP (Utilities|Struct|BreakS_Character _array_element)) (.Level (Utilities|Struct|BreakS_Character _array_element)) (.Level2 (Utilities|Struct|BreakS_Character _array_element)) (LocalVariables|GetUpdatedConditions) (.FortitudeSave (Utilities|Struct|BreakS_Character _array_element)) (.ReflexSave (Utilities|Struct|BreakS_Character _array_element)) (.ResolveSave (Utilities|Struct|BreakS_Character _array_element)) (.SpellSlotsCurrentL1 (Utilities|Struct|BreakS_Character _array_element)) (.SpellSlotsMaxL1 (Utilities|Struct|BreakS_Character _array_element)) (.SpellSlotsCurrentL2 (Utilities|Struct|BreakS_Character _array_element)) (.SpellSlotsMaxL2 (Utilities|Struct|BreakS_Character _array_element)) (.SpellSlotsCurrentL3 (Utilities|Struct|BreakS_Character _array_element)) (.SpellSlotsMaxL3 (Utilities|Struct|BreakS_Character _array_element)) (.SpellSlotsCurrentL4 (Utilities|Struct|BreakS_Character _array_element)) (.SpellSlotsMaxL4 (Utilities|Struct|BreakS_Character _array_element)) (.SpellSlotsCurrentL5 (Utilities|Struct|BreakS_Character _array_element)) (.SpellSlotsMaxL5 (Utilities|Struct|BreakS_Character _array_element)) (.SpellSlotsCurrentL6 (Utilities|Struct|BreakS_Character _array_element)) (.SpellSlotsMaxL6 (Utilities|Struct|BreakS_Character _array_element)) (.SpellSlotsCurrentL7 (Utilities|Struct|BreakS_Character _array_element)) (.SpellSlotsMaxL7 (Utilities|Struct|BreakS_Character _array_element)) (.MemorisedSpellsL1 (Utilities|Struct|BreakS_Character _array_element)) (.MemorisedSpellsL2 (Utilities|Struct|BreakS_Character _array_element)) (.MemorisedSpellsL3 (Utilities|Struct|BreakS_Character _array_element)) (.MemorisedSpellsL4 (Utilities|Struct|BreakS_Character _array_element)) (.MemorisedSpellsL5 (Utilities|Struct|BreakS_Character _array_element)) (.MemorisedSpellsL6 (Utilities|Struct|BreakS_Character _array_element)) (.MemorisedSpellsL7 (Utilities|Struct|BreakS_Character _array_element)) (.EquipWeapon (Utilities|Struct|BreakS_Character _array_element)) (.EquipShield (Utilities|Struct|BreakS_Character _array_element)) (.EquipArmour (Utilities|Struct|BreakS_Character _array_element)) (.EquipHelmet (Utilities|Struct|BreakS_Character _array_element)) (.EquipRing1 (Utilities|Struct|BreakS_Character _array_element)) (.EquipRing2 (Utilities|Struct|BreakS_Character _array_element)) (.EquipCloak (Utilities|Struct|BreakS_Character _array_element)) (.EquipMisc (Utilities|Struct|BreakS_Character _array_element)) (.Inventory (Utilities|Struct|BreakS_Character _array_element)) (.SkillPickPockets (Utilities|Struct|BreakS_Character _array_element)) (.SkillOpenLocks (Utilities|Struct|BreakS_Character _array_element)) (.SkillFindTraps (Utilities|Struct|BreakS_Character _array_element)) (.SkillRemoveTraps (Utilities|Struct|BreakS_Character _array_element)) (.SkillMoveSilently (Utilities|Struct|BreakS_Character _array_element)) (.SkillHideInShadows (Utilities|Struct|BreakS_Character _array_element)) (.SkillHearNoise (Utilities|Struct|BreakS_Character _array_element)) (.SkillClimbWalls (Utilities|Struct|BreakS_Character _array_element)) (.SkillReadLanguages (Utilities|Struct|BreakS_Character _array_element)) (.Protrait (Utilities|Struct|BreakS_Character _array_element)) (.IsPlayerControlled (Utilities|Struct|BreakS_Character _array_element)) (.CharacterID (Utilities|Struct|BreakS_Character _array_element))))
      (Default|CallOnPartyUpdated))))

(fn UpdateCharacterHP
  (params (CharacterID :type Integer) (NewHP :type Integer))
  (LocalVariables|SetInCharacterID CharacterID)
  (LocalVariables|SetInNewHP NewHP)
  (for (_array_element _array_index) (Variables|Default|GetPartyMembers)
    (if (== (LocalVariables|GetInCharacterID) (.CharacterID (Utilities|Struct|BreakS_Character _array_element)))
      (Utilities|Array|SetArrayElem (Variables|Default|GetPartyMembers) _array_index (Utilities|Struct|MakeS_Character (.CharacterName (Utilities|Struct|BreakS_Character _array_element)) (.Race (Utilities|Struct|BreakS_Character _array_element)) (.Class1 (Utilities|Struct|BreakS_Character _array_element)) (.Class2 (Utilities|Struct|BreakS_Character _array_element)) (.Morality (Utilities|Struct|BreakS_Character _array_element)) (.Gender (Utilities|Struct|BreakS_Character _array_element)) (.Might (Utilities|Struct|BreakS_Character _array_element)) (.Acuity (Utilities|Struct|BreakS_Character _array_element)) (.Resolve (Utilities|Struct|BreakS_Character _array_element)) (.Reflex (Utilities|Struct|BreakS_Character _array_element)) (.Vigor (Utilities|Struct|BreakS_Character _array_element)) (.Presence (Utilities|Struct|BreakS_Character _array_element)) (LocalVariables|GetInNewHP) (.MaxHP (Utilities|Struct|BreakS_Character _array_element)) (.DefenseRating (Utilities|Struct|BreakS_Character _array_element)) (.StrikeNumber (Utilities|Struct|BreakS_Character _array_element)) (.XP (Utilities|Struct|BreakS_Character _array_element)) (.Level (Utilities|Struct|BreakS_Character _array_element)) (.Level2 (Utilities|Struct|BreakS_Character _array_element)) (.Condition (Utilities|Struct|BreakS_Character _array_element)) (.FortitudeSave (Utilities|Struct|BreakS_Character _array_element)) (.ReflexSave (Utilities|Struct|BreakS_Character _array_element)) (.ResolveSave (Utilities|Struct|BreakS_Character _array_element)) (.SpellSlotsCurrentL1 (Utilities|Struct|BreakS_Character _array_element)) (.SpellSlotsMaxL1 (Utilities|Struct|BreakS_Character _array_element)) (.SpellSlotsCurrentL2 (Utilities|Struct|BreakS_Character _array_element)) (.SpellSlotsMaxL2 (Utilities|Struct|BreakS_Character _array_element)) (.SpellSlotsCurrentL3 (Utilities|Struct|BreakS_Character _array_element)) (.SpellSlotsMaxL3 (Utilities|Struct|BreakS_Character _array_element)) (.SpellSlotsCurrentL4 (Utilities|Struct|BreakS_Character _array_element)) (.SpellSlotsMaxL4 (Utilities|Struct|BreakS_Character _array_element)) (.SpellSlotsCurrentL5 (Utilities|Struct|BreakS_Character _array_element)) (.SpellSlotsMaxL5 (Utilities|Struct|BreakS_Character _array_element)) (.SpellSlotsCurrentL6 (Utilities|Struct|BreakS_Character _array_element)) (.SpellSlotsMaxL6 (Utilities|Struct|BreakS_Character _array_element)) (.SpellSlotsCurrentL7 (Utilities|Struct|BreakS_Character _array_element)) (.SpellSlotsMaxL7 (Utilities|Struct|BreakS_Character _array_element)) (.MemorisedSpellsL1 (Utilities|Struct|BreakS_Character _array_element)) (.MemorisedSpellsL2 (Utilities|Struct|BreakS_Character _array_element)) (.MemorisedSpellsL3 (Utilities|Struct|BreakS_Character _array_element)) (.MemorisedSpellsL4 (Utilities|Struct|BreakS_Character _array_element)) (.MemorisedSpellsL5 (Utilities|Struct|BreakS_Character _array_element)) (.MemorisedSpellsL6 (Utilities|Struct|BreakS_Character _array_element)) (.MemorisedSpellsL7 (Utilities|Struct|BreakS_Character _array_element)) (.EquipWeapon (Utilities|Struct|BreakS_Character _array_element)) (.EquipShield (Utilities|Struct|BreakS_Character _array_element)) (.EquipArmour (Utilities|Struct|BreakS_Character _array_element)) (.EquipHelmet (Utilities|Struct|BreakS_Character _array_element)) (.EquipRing1 (Utilities|Struct|BreakS_Character _array_element)) (.EquipRing2 (Utilities|Struct|BreakS_Character _array_element)) (.EquipCloak (Utilities|Struct|BreakS_Character _array_element)) (.EquipMisc (Utilities|Struct|BreakS_Character _array_element)) (.Inventory (Utilities|Struct|BreakS_Character _array_element)) (.SkillPickPockets (Utilities|Struct|BreakS_Character _array_element)) (.SkillOpenLocks (Utilities|Struct|BreakS_Character _array_element)) (.SkillFindTraps (Utilities|Struct|BreakS_Character _array_element)) (.SkillRemoveTraps (Utilities|Struct|BreakS_Character _array_element)) (.SkillMoveSilently (Utilities|Struct|BreakS_Character _array_element)) (.SkillHideInShadows (Utilities|Struct|BreakS_Character _array_element)) (.SkillHearNoise (Utilities|Struct|BreakS_Character _array_element)) (.SkillClimbWalls (Utilities|Struct|BreakS_Character _array_element)) (.SkillReadLanguages (Utilities|Struct|BreakS_Character _array_element)) (.Protrait (Utilities|Struct|BreakS_Character _array_element)) (.IsPlayerControlled (Utilities|Struct|BreakS_Character _array_element)) (.CharacterID (Utilities|Struct|BreakS_Character _array_element))))
      (Default|CallOnPartyUpdated))))

(fn LoadSavedParty
  (bind _returnvalue (SaveGame|DoesSaveGameExist "CharacterRoster"))
  (if _returnvalue
    (bind _returnvalue_2 (SaveGame|LoadGamefromSlot "CharacterRoster"))
    (bind _assg_character_roster (Utilities|Casting|CastToSG_CharacterRoster _returnvalue_2))
    (for _array_element (Variables|/Game/Blueprints/Data/SG_CharacterRoster.SG_CharacterRoster_C|GetSavedCharacters _assg_character_roster)
      (CallFunction|AddCharacter _array_element)
      (Default|CallOnPartyUpdated))))

(fn SavePartytoDisk
  (bind _returnvalue (SaveGame|DoesSaveGameExist "CharacterRoster"))
  (if _returnvalue
    (bind _returnvalue_2 (SaveGame|LoadGamefromSlot "CharacterRoster"))
    (bind _assg_character_roster (Utilities|Casting|CastToSG_CharacterRoster _returnvalue_2))
    (Utilities|Array|Add (Variables|/Game/Blueprints/Data/SG_CharacterRoster.SG_CharacterRoster_C|GetSavedCharacters _assg_character_roster) (Utilities|Array|Get(acopy) (Variables|Default|GetPartyMembers) (Utilities|Array|LastIndex (Variables|Default|GetPartyMembers))))
    (SaveGame|SaveGametoSlot _assg_character_roster "CharacterRoster")
    (else
      (bind _returnvalue_3 (SaveGame|CreateSaveGameObject "/Game/Blueprints/Data/SG_CharacterRoster.SG_CharacterRoster_C"))
      (bind _assg_character_roster_2 (Utilities|Casting|CastToSG_CharacterRoster _returnvalue_3))
      (Variables|/Game/Blueprints/Data/SG_CharacterRoster.SG_CharacterRoster_C|SetSavedCharacters _assg_character_roster_2 (Variables|Default|GetPartyMembers))
      (SaveGame|SaveGametoSlot _assg_character_roster_2 "CharacterRoster"))))