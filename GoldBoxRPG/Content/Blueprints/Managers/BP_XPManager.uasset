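; XP manager that handles monster XP rewards and character level-ups for the party, reached through BP_GameManager.
; AwardCombatXP looks up DT_Monsters values; DistributeXP splits a total among living members, then calls CheckLevelUp.
; CheckLevelUp tests the next class level's threshold and rolls hit dice plus Vigor bonus from DT_LevelProgression data.
; ApplyLevelUp posts a level message, but its ArraySet has no item connected, leaving the rebuilt character struct unused.
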(event EventBeginPlay)

(event Collision|EventActorBeginOverlap
  (params (OtherActor :type Actor%20Object%20Reference)))

(event EventTick
  (params (DeltaSeconds :type Float%20%28single-precision%29)))

(fn ConstructionScript)

(fn AwardCombatXP
  (params (MonsterGroupID :type Integer))
  (bind _returnvalue (Utilities|GetDataTableRow "/Game/Blueprints/Data/DT_Monsters.DT_Monsters" (Utilities|String|StringToName (Utilities|String|ToString(Text) (Utilities|Text|ToText(Integer) MonsterGroupID))))
    (:then
      (return (.XPValue (Utilities|Struct|BreakS_Monster _returnvalue))))
    (:RowNotFound
      (return 0))))

(fn DistributeXP
  (params (TotalXP :type Integer))
  (bind _asbp_game_manager (Utilities|Casting|CastToBP_GameManager (Game|GetGameInstance)))
  (if (> (Utilities|Array|Length (Default|GetLivingMembers (Variables|/Game/Blueprints/Core/BP_GameManager.BP_GameManager_C|GetPartyManager _asbp_game_manager))) 0)
    (LocalVariables|SetXPPerCharacter (/ TotalXP (Utilities|Array|Length (Default|GetLivingMembers (Variables|/Game/Blueprints/Core/BP_GameManager.BP_GameManager_C|GetPartyManager _asbp_game_manager)))))
    (for _array_element (Default|GetLivingMembers (Variables|/Game/Blueprints/Core/BP_GameManager.BP_GameManager_C|GetPartyManager _asbp_game_manager))
      (bind _asbp_game_manager_2 (Utilities|Casting|CastToBP_GameManager (Game|GetGameInstance)))
      (Default|AddXPtoCharacter (Variables|/Game/Blueprints/Core/BP_GameManager.BP_GameManager_C|GetPartyManager _asbp_game_manager_2) (.CharacterID (Utilities|Struct|BreakS_Character _array_element)) (LocalVariables|GetXPPerCharacter))
      (bind _asbp_game_manager_3 (Utilities|Casting|CastToBP_GameManager (Game|GetGameInstance)))
      (CallFunction|CheckLevelUp (Variables|/Game/Blueprints/Core/BP_GameManager.BP_GameManager_C|GetXPManagerRef _asbp_game_manager_3) (.CharacterID (Utilities|Struct|BreakS_Character _array_element))))))

(fn CheckLevelUp
  (params (CharacterID :type Integer))
  (bind _asbp_game_manager (Utilities|Casting|CastToBP_GameManager (Game|GetGameInstance)))
  (for _array_element (Variables|/Game/Blueprints/Managers/BP_PartyManager.BP_PartyManager_C|GetPartyMembers (Variables|/Game/Blueprints/Core/BP_GameManager.BP_GameManager_C|GetPartyManager _asbp_game_manager))
    (LocalVariables|SetNextLevel (+ (.Level (Utilities|Struct|BreakS_Character _array_element)) 1))
    (if (== (.CharacterID (Utilities|Struct|BreakS_Character _array_element)) CharacterID)
      (bind _returnvalue (Utilities|GetDataTableRow "/Game/Data/DataTables/DT_LevelProgression.DT_LevelProgression" (Utilities|String|StringToName (Utilities|String|Append (Utilities|String|EnumtoString (.Class1 (Utilities|Struct|BreakS_Character _array_element))) "_" (Utilities|String|ToString(Integer) (LocalVariables|GetNextLevel)))))
        (:then
          (bind _xprequired (CallFunction|GetXPThreshold (.Class1 (Utilities|Struct|BreakS_Character _array_element)) (LocalVariables|GetNextLevel)))
          (if (>= (.XP (Utilities|Struct|BreakS_Character _array_element)) _xprequired)
            (bind _total (CallFunction|DiceRoll 1 (.HitDiceType (Utilities|Struct|BreakS_LevelProgression _returnvalue))))
            (bind _hpbonus (CallFunction|GetVigorBonus (.Vigor (Utilities|Struct|BreakS_Character _array_element))))
            (LocalVariables|SetHPGained (+ _total _hpbonus))
            (bind _asbp_game_manager_2 (Utilities|Casting|CastToBP_GameManager (Game|GetGameInstance)))
            (CallFunction|ApplyLevelUp (Variables|/Game/Blueprints/Core/BP_GameManager.BP_GameManager_C|GetXPManagerRef _asbp_game_manager_2) CharacterID (LocalVariables|GetNextLevel) (.StrikeNumber (Utilities|Struct|BreakS_LevelProgression _returnvalue)) (LocalVariables|GetHPGained))))))))

(fn ApplyLevelUp
  (params (CharacterID :type Integer) (NewLevel :type Integer) (NewStrikeNumber :type Integer) (HPGained :type Integer))
  (bind _asbp_game_manager (Utilities|Casting|CastToBP_GameManager (Game|GetGameInstance)))
  (for (_array_element _array_index) (Variables|/Game/Blueprints/Managers/BP_PartyManager.BP_PartyManager_C|GetPartyMembers (Variables|/Game/Blueprints/Core/BP_GameManager.BP_GameManager_C|GetPartyManager _asbp_game_manager))
    (if (== (.CharacterID (Utilities|Struct|BreakS_Character _array_element)) CharacterID)
      (bind _asbp_game_manager_2 (Utilities|Casting|CastToBP_GameManager (Game|GetGameInstance)))
      (Utilities|Array|SetArrayElem :TargetArray (Variables|/Game/Blueprints/Managers/BP_PartyManager.BP_PartyManager_C|GetPartyMembers (Variables|/Game/Blueprints/Core/BP_GameManager.BP_GameManager_C|GetPartyManager _asbp_game_manager_2)) :Index _array_index)
      (bind _asbp_game_manager_3 (Utilities|Casting|CastToBP_GameManager (Game|GetGameInstance)))
      (Default|PostMessage (Variables|/Game/Blueprints/Core/BP_GameManager.BP_GameManager_C|GetTextManagerRef _asbp_game_manager_3) (Utilities|Text|ToText(String) (Utilities|String|Append (.CharacterName (Utilities|Struct|BreakS_Character _array_element)) " is now level " (Utilities|String|ToString(Integer) NewLevel))) "NewEnumerator2"))))