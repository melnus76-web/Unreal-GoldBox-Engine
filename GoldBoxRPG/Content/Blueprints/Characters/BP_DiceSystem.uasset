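; BP_DiceSystem provides tabletop-style dice rolls as three functions.
; Roll sums a given number of random integers, each from 1 to the die type, in RunningTotal and returns it.
; RollWithModifier adds a flat modifier to the result of Roll.
; PercentileRoll returns a single random integer from 1 to 100, independent of Roll.
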(fn Roll
  (params (NumDice :type Integer) (DieType :type Integer))
  (for _index (range 0 (- NumDice 1))
    (LocalVariables|SetRunningTotal (+ (LocalVariables|GetRunningTotal) (Math|Random|RandomIntegerinRange 1 DieType))))
  (return (LocalVariables|GetRunningTotal)))

(fn RollwithModifier
  (params (NumDice :type Integer) (DieType :type Integer) (Modifier :type Integer))
  (return (+ (CallFunction|Roll NumDice DieType) Modifier)))

(fn PercentileRoll
  (return (Math|Random|RandomIntegerinRange 1 100)))