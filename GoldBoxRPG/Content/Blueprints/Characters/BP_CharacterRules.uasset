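; BP_CharacterRules provides D&D-style character combat math: THAC0, descending armor class, Strength bonuses and saving throws.
; THAC0 and the five saving throws come from DT_LevelProgression and DT_SavingThrows, using row names built as Class_Level.
; AC subtracts Dexterity and magic bonuses from the base, while Strength maps to hit and damage bonuses through hardcoded brackets.
; Both table lookups handle only the Row Found path.
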(fn ComputeTHAC0
  (params (CharacterClass :type E_CharacterClass%20Enum :default "NewEnumerator0") (Level :type Integer))
  (bind _returnvalue (Utilities|GetDataTableRow "/Game/Data/DataTables/DT_LevelProgression.DT_LevelProgression" (Utilities|String|StringToName (Utilities|String|Append (Utilities|String|EnumtoString CharacterClass) (Utilities|String|MakeLiteralString "_") (Utilities|String|ToString(Integer) Level))))
    (:then
      (return (.THAC0 (Utilities|Struct|BreakS_LevelProgression _returnvalue))))))

(fn ComputeAC
  (params (BaseAC :type Integer) (DexBonus :type Integer) (MagicBonus :type Integer))
  (return (- (- BaseAC DexBonus) MagicBonus)))

(fn GetStrengthBonus
  (params (Strength :type Integer))
  (if (<= Strength 5)
    (LocalVariables|SetLocalHitBonus -2)
    (LocalVariables|SetLocalDamageBonus -1)
    (elif (<= Strength 8)
      (LocalVariables|SetLocalHitBonus -1)
      (LocalVariables|SetLocalDamageBonus 0)
      (elif (<= Strength 15)
        (LocalVariables|SetLocalHitBonus 0)
        (LocalVariables|SetLocalDamageBonus 0)
        (elif (== Strength 16)
          (LocalVariables|SetLocalHitBonus 0)
          (LocalVariables|SetLocalDamageBonus 1)
          (elif (== Strength 17)
            (LocalVariables|SetLocalHitBonus 1)
            (LocalVariables|SetLocalDamageBonus 1)
            (else
              (LocalVariables|SetLocalHitBonus 1)
              (LocalVariables|SetLocalDamageBonus 2)))))))
  (return (LocalVariables|GetLocalHitBonus) (LocalVariables|GetLocalDamageBonus)))

(fn ComputeSavingThrows
  (params (CharacterClass :type E_CharacterClass%20Enum :default "NewEnumerator0") (Level :type Integer))
  (bind _returnvalue (Utilities|GetDataTableRow "/Game/Data/DataTables/DT_SavingThrows.DT_SavingThrows" (Utilities|String|StringToName (Utilities|String|Append (Utilities|String|EnumtoString CharacterClass) (Utilities|String|MakeLiteralString "_") (Utilities|String|ToString(Integer) Level))))
    (:then
      (return (.VsPoison (Utilities|Struct|BreakS_SavingThrowRow _returnvalue)) (.VsWands (Utilities|Struct|BreakS_SavingThrowRow _returnvalue)) (.VsPetrification (Utilities|Struct|BreakS_SavingThrowRow _returnvalue)) (.VsBreath (Utilities|Struct|BreakS_SavingThrowRow _returnvalue)) (.VsSpells (Utilities|Struct|BreakS_SavingThrowRow _returnvalue))))))