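; BP_PartyManager is an actor that holds the party member list and answers queries about it.
; GetLivingMembers filters members by Condition, feeding the wipe check and the active speaker pick (first living member).
; ReorderParty writes two slots in sequence without a temporary, so both end up holding IndexB's member instead of swapping.
; AwardXPToParty is a stub that only prints a debug message.
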(event EventBeginPlay)

(event Collision|EventActorBeginOverlap
  (params (OtherActor :type Actor%20Object%20Reference)))

(event EventTick
  (params (DeltaSeconds :type Float%20%28single-precision%29)))

(fn ConstructionScript)

(fn AddCharacter
  (params (NewCharacter :type S%20Character%20Structure))
  (Utilities|Array|Add (Variables|Default|GetPartyMembers) NewCharacter))

(fn GetLivingMembers
  (for _array_element (Variables|Default|GetPartyMembers)
    (if (Utilities|Enum|NotEqual(Enum) (.Condition (Utilities|Struct|BreakS_Character _array_element)) "NewEnumerator10")
      (Utilities|Array|Add (LocalVariables|GetTempLiving) _array_element)))
  (return (LocalVariables|GetTempLiving)))

(fn IsPartyWiped
  (return (== (Utilities|Array|Length (CallFunction|GetLivingMembers)) 0)))

(fn GetActiveSpeaker
  (return (Utilities|Array|Get(acopy) (CallFunction|GetLivingMembers))))

(fn ReorderParty
  (params (IndexA :type Integer) (IndexB :type Integer))
  (bind _partymembers (Variables|Default|GetPartyMembers))
  (Utilities|Array|SetArrayElem _partymembers IndexA (Utilities|Array|Get(acopy) _partymembers IndexB))
  (Utilities|Array|SetArrayElem _partymembers IndexB (Utilities|Array|Get(acopy) _partymembers IndexA)))

(fn AwardXPtoParty
  (params (Amount :type Integer))
  (Development|PrintString "AwardXPToParty called"))