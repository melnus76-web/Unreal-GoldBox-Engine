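; Central game manager for a tile-based dungeon game with party, encounters and combat, holding game state, story flags and player tile position.
; Init, skipped in the test suite level, spawns and cross-wires the subsystem managers, creates a test party, then loads and generates the first map.
; LoadDungeonLevel loads a map, places the player and regenerates the dungeon, while state changes notify listeners.
; XP awards forward to the party manager; StartCombat and EndCombat are print-only stubs.
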(event EventInit
  (bind _returnvalue (Game|GetCurrentLevelName true))
  (if (not (Utilities|Enum|Equal(Enum) _returnvalue "L_TestSuite"))
    (CallFunction|InitialiseGameState)
    (CallFunction|SpawnManagers)
    (CallFunction|InitialiseParty)
    (CallFunction|InitialiseWorld)))

(fn ChangeGameState
  (params (NewState :type E_GameState%20Enum :default "NewEnumerator0"))
  (bind _output_get (Variables|Default|SetCurrentGameState NewState))
  (Default|CallOnGameStateChanged _output_get)
  (Default|CallOnGameStateUpdated _output_get))

(fn SetStoryFlag
  (params (FlagName :type String) (Value :type Boolean))
  (Utilities|Map|Add (Variables|Default|GetStoryFlags) FlagName Value))

(fn CheckStoryFlag
  (params (FlagName :type String))
  (return (.ReturnValue (Utilities|Map|Find (Variables|Default|GetStoryFlags) FlagName))))

(fn LoadDungeonLevel
  (params (LevelId :type Integer) (EntryTileX :type Integer) (EntryTIleY :type Integer))
  (bind _dungeongeneratorref (Variables|Default|GetDungeonGeneratorRef))
  (Utilities|FlowControl|Sequence
    (:then_0
      (Variables|Default|SetCurrentDungeonLevelID LevelId)
      (Default|LoadMap (Variables|Default|GetMapManagerRef) LevelId)
      (Variables|Default|SetCurrentPlayerTileX EntryTileX)
      (Variables|Default|SetCurrentPlayerTileY EntryTIleY)
      (Default|UpdatePlayerPosition (Variables|Default|GetMapManagerRef) EntryTileX EntryTIleY)
      (Utilities|IsValid _dungeongeneratorref
        (:Is%20Valid
          (Default|GenerateDungeon _dungeongeneratorref)
          (CallFunction|ChangeGameState (Utilities|Enum|LiteralenumE_GameState "NewEnumerator1")))))))

(fn StartCombat
  (Development|PrintString "StartCombat called"))

(fn EndCombat
  (params (Victory :type Boolean))
  (Development|PrintString "EndCombat called"))

(fn AwardXP
  (params (Amount :type Integer))
  (Default|AwardXPtoParty (Variables|Default|GetPartyManager) Amount))

(fn InitialiseGameState
  (Variables|Default|SetCurrentGameState "NewEnumerator0"))

(fn SpawnManagers
  (bind _returnvalue (Game|GetCurrentLevelName true))
  ;[0.15 0.15 0.15 0.5] Party Manager
  (if (not (Utilities|Enum|Equal(Enum) _returnvalue "L_TestSuite"))
    (bind _returnvalue_2 (Game|SpawnActorfromClass "/Game/Blueprints/Managers/BP_PartyManager.BP_PartyManager_C" (Math|Transform|MakeTransform "0, 0, 0" "0, 0, 0" "1.000000,1.000000,1.000000") "Undefined" "MultiplyWithRoot" 0 0))
    ;[0.15 0.15 0.15 0.5] Map Manager
    (Variables|Default|SetPartyManager _returnvalue_2)
    (bind _returnvalue_3 (Game|SpawnActorfromClass "/Game/Blueprints/Dungeon/BP_MapManager.BP_MapManager_C" (Math|Transform|MakeTransform "0, 0, 0" "0, 0, 0" "1.000000,1.000000,1.000000") "Undefined" "MultiplyWithRoot" 0 0))
    (Variables|Default|SetMapManagerRef _returnvalue_3)
    (bind _returnvalue_4 (Game|SpawnActorfromClass "/Game/Blueprints/Managers/BP_TextManager.BP_TextManager_C" (Math|Transform|MakeTransform "0, 0, 0" "0, 0, 0" "1.000000,1.000000,1.000000") "Undefined" "MultiplyWithRoot" 0 0))
    (Variables|Default|SetTextManagerRef _returnvalue_4)
    (bind _returnvalue_5 (Game|SpawnActorfromClass "/Game/Blueprints/Managers/BP_EventManager.BP_EventManager_C" (Math|Transform|MakeTransform "0, 0, 0" "0, 0, 0" "1.000000,1.000000,1.000000") "Undefined" "MultiplyWithRoot" 0 0))
    (Variables|Default|SetEventManagerRef _returnvalue_5)
    (Variables|/Game/Blueprints/Managers/BP_EventManager.BP_EventManager_C|SetMapManagerRef (Variables|Default|GetEventManagerRef) (Variables|Default|GetMapManagerRef))
    (Variables|/Game/Blueprints/Managers/BP_EventManager.BP_EventManager_C|SetTextManagerRef (Variables|Default|GetEventManagerRef) (Variables|Default|GetTextManagerRef))
    (bind _returnvalue_6 (Game|SpawnActorfromClass "/Game/Blueprints/Dungeon/BP_DungeonGenerator.BP_DungeonGenerator_C" (Math|Transform|MakeTransform "0, 0, 0" "0, 0, 0" "1.000000,1.000000,1.000000") "Undefined" "MultiplyWithRoot" 0 0))
    (Variables|Default|SetDungeonGeneratorRef _returnvalue_6)
    (bind _returnvalue_7 (Game|SpawnActorfromClass "/Game/Blueprints/Managers/BP_EncounterManager.BP_EncounterManager_C" (Math|Transform|MakeTransform "0, 0, 0" "0, 0, 0" "1.000000,1.000000,1.000000") "Undefined" "MultiplyWithRoot" 0 0))
    (bind _output_get (Variables|Default|SetEncounterManagerRef _returnvalue_7))
    (Variables|/Game/Blueprints/Managers/BP_EncounterManager.BP_EncounterManager_C|SetTextManagerRef _output_get (Variables|Default|GetTextManagerRef))
    (Variables|/Game/Blueprints/Managers/BP_EncounterManager.BP_EncounterManager_C|SetGameManagerRef (Variables|Default|GetEncounterManagerRef) self)
    (bind _returnvalue_8 (Game|SpawnActorfromClass "/Game/Blueprints/Combat/BP_CombatManager.BP_CombatManager_C" (Math|Transform|MakeTransform "0, 0, 0" "0, 0, 0" "1.000000,1.000000,1.000000") "Undefined" "MultiplyWithRoot" 0 0))
    (bind _output_get_2 (Variables|Default|SetCombatManagerRef _returnvalue_8))
    (Variables|/Game/Blueprints/Combat/BP_CombatManager.BP_CombatManager_C|SetGameManagerRef _output_get_2 self)
    (Variables|/Game/Blueprints/Combat/BP_CombatManager.BP_CombatManager_C|SetTextManagerRef (Variables|Default|GetCombatManagerRef) (Variables|Default|GetTextManagerRef))
    (Variables|/Game/Blueprints/Combat/BP_CombatManager.BP_CombatManager_C|SetPartyManagerRef (Variables|Default|GetCombatManagerRef) (Variables|Default|GetPartyManager))
    (bind _returnvalue_9 (Game|SpawnActorfromClass "/Game/Blueprints/Combat/BP_EnemyAI.BP_EnemyAI_C" (Math|Transform|MakeTransform "0, 0, 0" "0, 0, 0" "1.000000,1.000000,1.000000") "Undefined" "MultiplyWithRoot" 0 0))
    (Variables|Default|SetEnemyAIRef _returnvalue_9)
    (bind _returnvalue_10 (Game|SpawnActorfromClass "/Game/Blueprints/Managers/BP_XPManager.BP_XPManager_C" (Math|Transform|MakeTransform "0, 0, 0" "0, 0, 0" "1.000000,1.000000,1.000000") "Undefined" "MultiplyWithRoot" 0 0))
    (Variables|Default|SetXPManagerRef _returnvalue_10)))

(fn InitialiseParty
  (Default|InitialiseTestParty (Variables|Default|GetPartyManager)))

(fn InitialiseWorld
  (Default|LoadMap (Variables|Default|GetMapManagerRef) 1)
  (bind _outactors (Actor|GetAllActorsOfClass "/Game/Blueprints/Dungeon/BP_DungeonGenerator.BP_DungeonGenerator_C"))
  (Variables|Default|SetDungeonGeneratorRef (Utilities|Array|Get(acopy) _outactors))
  (Variables|/Game/Blueprints/Dungeon/BP_DungeonGenerator.BP_DungeonGenerator_C|SetMapManager (Variables|Default|GetDungeonGeneratorRef) (Variables|Default|GetMapManagerRef))
  (Default|GenerateDungeon (Variables|Default|GetDungeonGeneratorRef)))