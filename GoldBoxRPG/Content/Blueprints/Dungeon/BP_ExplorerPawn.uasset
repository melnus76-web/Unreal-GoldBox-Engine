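; Player pawn for grid-based dungeon exploration, moving one tile forward or back and turning in instant 90-degree steps via Enhanced Input.
; MapManager wall and passability checks gate each move, then a timeline lerps between tile centers while input is locked.
; On arrival it updates the map and GameManager position, evaluates EventManager tile triggers, increments the step counter and unlocks.
; A separate timeline animates its point light intensity.
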(event Custom|MoveForward)

(event Input|EnhancedActionEvents|EnhancedInputActionIA_MoveForward
  (params (ActionValue :type Boolean) (ElapsedSeconds :type Float%20%28double-precision%29) (TriggeredSeconds :type Float%20%28double-precision%29) (InputAction :type Input%20Action%20Object%20Reference :default "/Game/Input/IA_MoveForward.IA_MoveForward"))
  ;[0.15 0.15 0.15 0.5] Move Forward
  (:Started
    (CallFunction|MoveForward)
    (bind _canmove (CallFunction|CanInitiateMove (Variables|Default|GetFacingDirection)))
    (if _canmove
      (CallFunction|PrepareMovement (Variables|Default|GetFacingDirection))
      ;[0.15 0.15 0.15 0.5] Move Visuals
      (bind _alpha (Timeline|MovementTimeline PlayFromStart)
        (:Update
          (Transformation|SetActorLocation (Math|Vector|Lerp(Vector) (Variables|Default|GetStartLocation) (Variables|Default|GetEndLocation) _alpha) false false))
        (:Finished
          (Development|PrintString "Movement End" true true "(R=0.000000,G=1.000000,B=0.038291,A=1.000000)")
          (CallFunction|CompleteMovement))))))

(event Input|EnhancedActionEvents|EnhancedInputActionIA_MoveBackward
  (params (ActionValue :type Boolean) (ElapsedSeconds :type Float%20%28double-precision%29) (TriggeredSeconds :type Float%20%28double-precision%29) (InputAction :type Input%20Action%20Object%20Reference :default "/Game/Input/IA_MoveBackward.IA_MoveBackward"))
  (bind _facingdirection (Variables|Default|GetFacingDirection))
  (bind _opposite (CallFunction|GetOppositeDirection _facingdirection))
  ;[0.15 0.15 0.15 0.5] Move Backwards
  (:Started
    (if (CallFunction|CanInitiateMove _opposite)
      (CallFunction|PrepareMovement _opposite)
      ;[0.15 0.15 0.15 0.5] Move Visuals
      (bind _alpha (Timeline|MovementTimeline PlayFromStart)
        (:Update
          (Transformation|SetActorLocation (Math|Vector|Lerp(Vector) (Variables|Default|GetStartLocation) (Variables|Default|GetEndLocation) _alpha) false false))
        (:Finished
          (Development|PrintString "Movement End" true true "(R=0.000000,G=1.000000,B=0.038291,A=1.000000)")
          (CallFunction|CompleteMovement))))))

(event Input|EnhancedActionEvents|EnhancedInputActionIA_TurnLeft
  (params (ActionValue :type Boolean) (ElapsedSeconds :type Float%20%28double-precision%29) (TriggeredSeconds :type Float%20%28double-precision%29) (InputAction :type Input%20Action%20Object%20Reference :default "/Game/Input/IA_TurnLeft.IA_TurnLeft"))
  ;[0.15 0.15 0.15 0.5] Turn Left
  (:Started
    (if (not (Variables|Default|GetIsMovementLocked))
      (switch Utilities|FlowControl|Switch|SwitchonE_Direction (Variables|Default|GetFacingDirection)
        (:NewEnumerator0
          (Variables|Default|SetFacingDirection "NewEnumerator3"))
        (:NewEnumerator1
          (Variables|Default|SetFacingDirection "NewEnumerator0"))
        (:NewEnumerator2
          (Variables|Default|SetFacingDirection "NewEnumerator1"))
        (:NewEnumerator3
          (Variables|Default|SetFacingDirection "NewEnumerator2")))
      (CallFunction|ApplyFacingRotation))))

(event Input|EnhancedActionEvents|EnhancedInputActionIA_TurnRight
  (params (ActionValue :type Boolean) (ElapsedSeconds :type Float%20%28double-precision%29) (TriggeredSeconds :type Float%20%28double-precision%29) (InputAction :type Input%20Action%20Object%20Reference :default "/Game/Input/IA_TurnRight.IA_TurnRight"))
  ;[0.15 0.15 0.15 0.5] Turn Right
  (:Started
    (if (not (Variables|Default|GetIsMovementLocked))
      (switch Utilities|FlowControl|Switch|SwitchonE_Direction (Variables|Default|GetFacingDirection)
        (:NewEnumerator0
          (Variables|Default|SetFacingDirection "NewEnumerator1"))
        (:NewEnumerator1
          (Variables|Default|SetFacingDirection "NewEnumerator2"))
        (:NewEnumerator2
          (Variables|Default|SetFacingDirection "NewEnumerator3"))
        (:NewEnumerator3
          (Variables|Default|SetFacingDirection "NewEnumerator0")))
      (CallFunction|ApplyFacingRotation))))

(event EventBeginPlay
  (bind _returnvalue (Game|GetPlayerController 0))
  (bind _gridx (Variables|Default|GetGridX))
  (bind _gridy (Variables|Default|GetGridY))
  (Input|SetInputModeGameOnly _returnvalue false)
  (Variables|/Script/Engine.PlayerController|SetbEnableClickEvents _returnvalue true)
  (Variables|/Script/Engine.PlayerController|SetbShowMouseCursor _returnvalue true)
  (bind _asbp_game_manager (Utilities|Casting|CastToBP_GameManager (Game|GetGameInstance)))
  (Variables|Default|SetMapManager (Variables|/Game/Blueprints/Core/BP_GameManager.BP_GameManager_C|GetMapManagerRef _asbp_game_manager))
  (Default|UpdatePlayerPosition (Variables|Default|GetMapManager) _gridx _gridy)
  (Transformation|SetActorLocation (Math|Vector|MakeVector (Math|Conversions|ToFloat(Integer) (* _gridx 400)) (Math|Conversions|ToFloat(Integer) (* _gridy 400)) 0.0) false false)
  (Transformation|SetActorRotation (Math|Rotator|MakeRotator 0.0 0.0 0.0))
  (Development|PrintString "ExplorerPaen ready at 0, 3 facing North")
  (Input|AddMappingContext (PlayerController|LocalPlayerSubsystems|GetEnhancedInputLocalPlayerSubsystem (Game|GetPlayerController 0)) "/Game/Input/IMC_Dungeon.IMC_Dungeon" 0 "(bIgnoreAllPressedKeysUntilRelease=True,bForceImmediately=False,bNotifyUserSettings=False)")
  (Development|PrintString "Mapping COntext initialised")
  (CallFunction|ApplyFacingRotation)
  (bind _intensity (Timeline|Timeline Play)
    (:Update
      (Rendering|Components|Light|SetIntensity (Variables|Default|GetPointLight) (* _intensity 4.0)))))

(fn ConstructionScript)

(fn GetTargetTile
  (params (FromX :type Integer) (FromY :type Integer) (Direction :type E_Direction%20Enum :default "NewEnumerator0"))
  (switch Utilities|FlowControl|Switch|SwitchonE_Direction Direction
    (:NewEnumerator0
      (LocalVariables|SetResultX FromX)
      (LocalVariables|SetResultY (- FromY 1)))
    (:NewEnumerator1
      (LocalVariables|SetResultX (+ FromX 1))
      (LocalVariables|SetResultY FromY))
    (:NewEnumerator2
      (LocalVariables|SetResultX FromX)
      (LocalVariables|SetResultY (+ FromY 1)))
    (:NewEnumerator3
      (LocalVariables|SetResultX (- FromX 1))
      (LocalVariables|SetResultY FromY)))
  (return (LocalVariables|GetResultX) (LocalVariables|GetResultY)))

(fn CanMoveto
  (params (TileX :type Integer) (TileY :type Integer))
  (return (.Passable (Utilities|Struct|BreakS_DungeonTile (Default|GetTile (Variables|Default|GetMapManager) TileX TileY)))))

(fn GridtoWorldLocation
  (params (TileX :type Integer) (TileY :type Integer))
  (return (Math|Vector|MakeVector (Math|Conversions|ToFloat(Integer) (* TileX 400)) (Math|Conversions|ToFloat(Integer) (* TileY 400)) 0.0)))

(fn CanInitiateMove
  (params (MoveDirection :type E_Direction%20Enum :default "NewEnumerator0"))
  (bind _gridx (Variables|Default|GetGridX))
  (bind _gridy (Variables|Default|GetGridY))
  (bind (_targetx _targety) (CallFunction|GetTargetTile _gridx _gridy MoveDirection))
  (bind _output_get (Variables|Default|SetCanMove true))
  (if _output_get
    (if (not (Variables|Default|GetIsMovementLocked))
      (if (not (Default|CheckWall (Variables|Default|GetMapManager) (Variables|Default|GetGridX) (Variables|Default|GetGridY) MoveDirection))
        (if (CallFunction|CanMoveto _targetx _targety)
          (bind _output_get_2 (Variables|Default|SetCanMove true))
          (else
            (Variables|Default|SetCanMove false :!label _label)))
        (else
          (goto _label)))
      (else
        (goto _label)))
    (else
      (goto _label)))
  (return _output_get_2))

(fn PrepareMovement
  (params (MoveDirection :type E_Direction%20Enum :default "NewEnumerator0"))
  (bind _gridx (Variables|Default|GetGridX))
  (bind _gridy (Variables|Default|GetGridY))
  (bind (_targetx _targety) (CallFunction|GetTargetTile _gridx _gridy MoveDirection))
  (bind _output_get (Variables|Default|SetTargetTileX _targetx))
  (bind _output_get_2 (Variables|Default|SetTargetTileY _targety))
  (Variables|Default|SetStartLocation (CallFunction|GridtoWorldLocation _gridx _gridy))
  (Variables|Default|SetEndLocation (CallFunction|GridtoWorldLocation _output_get _output_get_2))
  (Variables|Default|SetIsMovementLocked true))

(fn CompleteMovement
  (Variables|Default|SetGridX (Variables|Default|GetTargetTileX))
  (Variables|Default|SetGridY (Variables|Default|GetTargetTileY))
  ;[0.15 0.15 0.15 0.5] Comment
  (Default|UpdatePlayerPosition (Variables|Default|GetMapManager) (Variables|Default|GetGridX) (Variables|Default|GetGridY))
  (bind _asbp_game_manager (Utilities|Casting|CastToBP_GameManager (Game|GetGameInstance)))
  (Variables|/Game/Blueprints/Core/BP_GameManager.BP_GameManager_C|SetCurrentPlayerTileX _asbp_game_manager (Variables|Default|GetGridX))
  (Variables|/Game/Blueprints/Core/BP_GameManager.BP_GameManager_C|SetCurrentPlayerTileY _asbp_game_manager (Variables|Default|GetGridY))
  (Default|EvaluateTriggers (Variables|/Game/Blueprints/Core/BP_GameManager.BP_GameManager_C|GetEventManagerRef _asbp_game_manager) (Variables|Default|GetGridX) (Variables|Default|GetGridY) "NewEnumerator0")
  (Default|IncrementStepCounter (Variables|Default|GetMapManager))
  (Variables|Default|SetIsMovementLocked false))

(fn ApplyFacingRotation
  (Transformation|SetActorRotation (CallFunction|GetFacingRotation (Variables|Default|GetFacingDirection))))