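; Dungeon generator actor that builds the level geometry from the current map held by the GameManager's MapManager.
; On BeginPlay it walks every tile row by row and, for each passable tile, places a floor, a ceiling and walls according to the tile's per-side flags.
; All pieces are world-space instances on floor, ceiling and wall instanced mesh components, with wall offsets hardcoded rather than derived from TileSize.
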(event EventBeginPlay
  (bind _asbp_game_manager (Utilities|Casting|CastToBP_GameManager (Game|GetGameInstance)))
  (Variables|Default|SetMapManager (Variables|/Game/Blueprints/Core/BP_GameManager.BP_GameManager_C|GetMapManagerRef _asbp_game_manager))
  (if (Utilities|IsValid (Variables|Default|GetMapManager))
    (CallFunction|GenerateDungeon)))

(fn ConstructionScript)

(fn TiletoWorldLocation
  (params (TileX :type Integer) (TileY :type Integer))
  (bind _tilesize (Variables|Default|GetTileSize))
  (bind _output_get (LocalVariables|SetWorldX (* TileX _tilesize)))
  (bind _output_get_2 (LocalVariables|SetWorldY (* TileY _tilesize)))
  (return (Math|Vector|MakeVector _output_get _output_get_2 0.0)))

(fn GenerateDungeon
  (for _index (range 0 (- (.Height (Utilities|Struct|BreakS_DungeonMap (Variables|/Game/Blueprints/Dungeon/BP_MapManager.BP_MapManager_C|GetCurrentMap (Variables|Default|GetMapManager)))) 1))
    (CallFunction|ProcessRow _index)))

(fn SpawnNorthWall
  (params (TileX :type Integer) (TileY :type Integer))
  (bind _location (CallFunction|TiletoWorldLocation TileX TileY))
  (Components|InstancedStaticMesh|AddInstance (Variables|Default|GetWallMeshComponent) (Math|Transform|MakeTransform (Math|Vector|MakeVector (.x _location) (- (.y _location) 2e+02) 0.0) (Math|Rotator|MakeRotator 0.0 0.0 9e+01)) true))

(fn SpawnEastWall
  (params (TileX :type Integer) (TileY :type Integer))
  (bind _location (CallFunction|TiletoWorldLocation TileX TileY))
  (Components|InstancedStaticMesh|AddInstance (Variables|Default|GetWallMeshComponent) (Math|Transform|MakeTransform (Math|Vector|MakeVector (+ (.x _location) 2e+02) (.y _location) 0.0)) true))

(fn SpawnSouthWall
  (params (TileX :type Integer) (TileY :type Integer))
  (bind _location (CallFunction|TiletoWorldLocation TileX TileY))
  (Components|InstancedStaticMesh|AddInstance (Variables|Default|GetWallMeshComponent) (Math|Transform|MakeTransform (Math|Vector|MakeVector (.x _location) (+ (.y _location) 2e+02) 0.0) (Math|Rotator|MakeRotator 0.0 0.0 9e+01)) true))

(fn SpawnWestWall
  (params (TileX :type Integer) (TileY :type Integer))
  (bind _location (CallFunction|TiletoWorldLocation TileX TileY))
  (Components|InstancedStaticMesh|AddInstance (Variables|Default|GetWallMeshComponent) (Math|Transform|MakeTransform (Math|Vector|MakeVector (- (.x _location) 2e+02) (.y _location) 0.0)) true))

(fn SpawnFloorandCeiling
  (params (TileX :type Integer) (TileY :type Integer))
  (CallFunction|AddFloorInstance TileX TileY)
  (CallFunction|AddCeilingInstance TileX TileY))

(fn AddFloorInstance
  (params (TileX :type Integer) (TileY :type Integer))
  (bind _location (CallFunction|TiletoWorldLocation TileX TileY))
  (Components|InstancedStaticMesh|AddInstance (Variables|Default|GetFloorMeshComponent) (Math|Transform|MakeTransform (Math|Vector|MakeVector (.X (Math|Vector|BreakVector _location)) (.Y (Math|Vector|BreakVector _location)) 0.0) (Math|Rotator|MakeRotator 0.0 0.0 0.0) (Math|Vector|MakeVector 1.0 1.0 1.0)) true))

(fn AddCeilingInstance
  (params (TileX :type Integer) (TileY :type Integer))
  (bind _location (CallFunction|TiletoWorldLocation TileX TileY))
  (Components|InstancedStaticMesh|AddInstance (Variables|Default|GetCeilingMeshComponent) (Math|Transform|MakeTransform (Math|Vector|MakeVector (.X (Math|Vector|BreakVector _location)) (.Y (Math|Vector|BreakVector _location)) (Variables|Default|GetWallHeight)) (Math|Rotator|MakeRotator 0.0 0.0 0.0) (Math|Vector|MakeVector 1.0 1.0 1.0)) true))

(fn ProcessRow
  (params (RowIndex :type Integer))
  (for _index (range 0 (- (.Width (Utilities|Struct|BreakS_DungeonMap (Variables|/Game/Blueprints/Dungeon/BP_MapManager.BP_MapManager_C|GetCurrentMap (Variables|Default|GetMapManager)))) 1))
    (CallFunction|ProcessTile _index RowIndex)))

(fn ProcessTile
  (params (TileX :type Integer) (TileY :type Integer))
  (bind _mapmanager (Variables|Default|GetMapManager))
  (bind _tile (Default|GetTile _mapmanager TileX TileY))
  (bind (_wallnorth _walleast _wallsouth _wallwest _doornorth _dooreast _doorsouth _doorwest _passable) (Utilities|Struct|BreakS_DungeonTile _tile))
  (if _passable
    (CallFunction|SpawnFloorandCeiling TileX TileY)
    (CallFunction|SpawnTileWalls TileX TileY _wallnorth _walleast _wallsouth _wallwest)))

(fn SpawnTileWalls
  (params (TileX :type Integer) (TileY :type Integer) (WallN :type Boolean) (WallE :type Boolean) (WallS :type Boolean) (WallW :type Boolean))
  (if WallN
    (CallFunction|SpawnNorthWall TileX TileY))
  (if WallE
    (CallFunction|SpawnEastWall TileX TileY))
  (if WallS
    (CallFunction|SpawnSouthWall TileX TileY))
  (if WallW
    (CallFunction|SpawnWestWall TileX TileY)))