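; Dungeon map manager that holds the current level's tile grid and tracks player tile position and step count.
; LoadMap takes map data from an asset and fills a flat grid with impassable tiles, falling back to a hard-coded test corridor.
; Tile and door queries index that grid, while GetExitTile searches CurrentMap's own; CheckWall's logic is unwired.
; Level transitions resolve stair target IDs and hand off to BP_GameManager.
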(event EventBeginPlay
  (Development|PrintString "GenerateTestMap called"))

(event Collision|EventActorBeginOverlap
  (params (OtherActor :type Actor%20Object%20Reference)))

(event EventTick
  (params (DeltaSeconds :type Float%20%28single-precision%29)))

(fn ConstructionScript)

(fn GenerateTestMap
  (Variables|Default|SetCurrentMap (Utilities|Struct|MakeS_DungeonMap 1 8))
  (Variables|Default|SetIsMapLoaded true)
  (Variables|Default|SetCurrentLevelID 1)
  (CallFunction|FillMapwithEmptyTiles)
  (CallFunction|AddTiletoMap 0 3 true "NewEnumerator0" 0 0 false true false true true)
  (CallFunction|AddTiletoMap 1 3 true "NewEnumerator0" 0 0 false true false true false)
  (CallFunction|AddTiletoMap 2 3 true "NewEnumerator0" 0 0 false true false true false)
  (CallFunction|AddTiletoMap 3 3 true "NewEnumerator0" 2 2 false true false true false)
  (CallFunction|AddTiletoMap 4 3 true "NewEnumerator0" 0 1 false true false true false)
  (CallFunction|AddTiletoMap 5 3 true "NewEnumerator0" 0 0 false true true false false)
  (CallFunction|AddTiletoMap 5 4 true "NewEnumerator0" 0 0 false false true false true)
  (CallFunction|AddTiletoMap 5 5 true "NewEnumerator0" 0 0 false false true false true)
  (CallFunction|AddTiletoMap 5 6 true "NewEnumerator0" 0 0 true false true true true)
  (Variables|Default|SetCurrentMap ""))

(fn AddTiletoMap
  (params (TileX :type Integer) (TileY :type Integer) (bPassable :type Boolean) (TileType :type E_TileType%20Enum :default "NewEnumerator0") (MessageID :type Integer) (EventTriggerID :type Integer) (bIsExit :type Boolean) (WallNorth :type Boolean) (WallEast :type Boolean) (WallSouth :type Boolean) (WallWest :type Boolean))
  (Utilities|Array|SetArrayElem (Variables|Default|GetTileGrid) (+ (* TileY (.Width (Utilities|Struct|BreakS_DungeonMap (Variables|Default|GetCurrentMap)))) TileX) (Utilities|Struct|MakeS_DungeonTile WallNorth WallEast WallSouth WallWest false false false false bPassable TileType EventTriggerID MessageID false false false bIsExit)))

(fn LoadMap
  (params (MapDataAsset :type BP%20Dungeon%20Map%20Data%20Object%20Reference))
  (if (Utilities|IsValid MapDataAsset)
    (Variables|Default|SetCurrentMap (Variables|/Game/Blueprints/Dungeon/BP_DungeonMapData.BP_DungeonMapData_C|GetMapData MapDataAsset))
    (Variables|Default|SetCurrentLevelID (.LevelID (Utilities|Struct|BreakS_DungeonMap (Variables|Default|GetCurrentMap))))
    (CallFunction|FillMapwithEmptyTiles)
    (Variables|Default|SetCurrentLevelID (Variables|Default|GetCurrentLevelID))
    (Variables|Default|SetIsMapLoaded true)
    (else
      (CallFunction|GenerateTestMap)
      (Variables|Default|SetCurrentLevelID (Variables|Default|GetCurrentLevelID))
      (Variables|Default|SetIsMapLoaded true))))

(fn GetTile
  (params (TileX :type Integer) (TileY :type Integer))
  (return (Utilities|Array|Get(acopy) (Variables|Default|GetTileGrid) (+ TileX (* TileY (.Width (Utilities|Struct|BreakS_DungeonMap (Variables|Default|GetCurrentMap))))))))

(fn CheckWall
  (params (TileX :type Integer) (TileY :type Integer) (Direction :type E_Direction%20Enum :default "NewEnumerator0")))

(fn CheckDoor
  (params (TileX :type Integer) (TileY :type Integer) (Direction :type E_Direction%20Enum :default "NewEnumerator0"))
  (bind _tile (CallFunction|GetTile TileX TileY))
  (bind (_wallnorth _walleast _wallsouth _wallwest _doornorth _dooreast _doorsouth _doorwest) (Utilities|Struct|BreakS_DungeonTile _tile))
  (switch Utilities|FlowControl|Switch|SwitchonE_Direction Direction
    (:NewEnumerator0
      (LocalVariables|SetResult _doornorth))
    (:NewEnumerator1
      (LocalVariables|SetResult _dooreast))
    (:NewEnumerator2
      (LocalVariables|SetResult _doorsouth))
    (:NewEnumerator3
      (LocalVariables|SetResult _doorwest)))
  (return (LocalVariables|GetResult)))

(fn UpdatePlayerPosition
  (params (NewX :type Integer) (NewY :type Integer))
  (Variables|Default|SetPlayerTIleX NewX)
  (Variables|Default|SetPlayerTileY NewY))

(fn GetExitTile
  (bind _currentmap (Variables|Default|GetCurrentMap))
  (bind (_levelid _width _height _tilegrid) (Utilities|Struct|BreakS_DungeonMap _currentmap))
  (for (_array_element _array_index) _tilegrid
    (if (.IsExitTile (Utilities|Struct|BreakS_DungeonTile _array_element))
      (LocalVariables|SetExitX (Math|Integer|%(Integer) _array_index _width))
      (LocalVariables|SetExitY (/ _array_index _width))
      (return (Math|Vector2D|MakeVector2D (Math|Conversions|ToFloat(Integer) (LocalVariables|GetExitX)) (Math|Conversions|ToFloat(Integer) (LocalVariables|GetExitY)))))))

(fn IncrementStepCounter
  (params (EncounterType :type Integer))
  (Variables|Default|SetStepCounter (+ (Variables|Default|GetStepCounter) 1)))

(fn HandleLevelTransition
  (params (GoingUp :type Boolean))
  (bind _targetlevelid (CallFunction|ResolveTransitionTargetLevelID GoingUp))
  (if (!= _targetlevelid -1)
    (bind _asbp_game_manager (Utilities|Casting|CastToBP_GameManager (Game|GetGameInstance)))
    (Default|LoadDungeonLevel _asbp_game_manager _targetlevelid (Variables|Default|GetPlayerTIleX) (Variables|Default|GetPlayerTileY))
    (else
      (Development|PrintString "No transition defined in this direction"))))

(fn FillMapwithEmptyTiles
  (bind _currentmap (Variables|Default|GetCurrentMap))
  (bind (_levelid _width _height) (Utilities|Struct|BreakS_DungeonMap _currentmap))
  (for _index (range 0 (- (* _width _height) 1))
    (Utilities|Array|Add (Variables|Default|GetTileGrid) (Utilities|Struct|MakeS_DungeonTile false false false false false false false false false))))

(fn ResolveTransitionTargetLevelID
  (params (GoingUp :type Boolean))
  (bind _currentmap (Variables|Default|GetCurrentMap))
  (bind (_levelid _width _height _tilegrid _stepcounterthresholds _randomencountertableid _ambientlighting _stairsuptargetlevelid _stairsdowntargetlevelid) (Utilities|Struct|BreakS_DungeonMap _currentmap))
  (if GoingUp
    (return _stairsuptargetlevelid)
    (else
      (return _stairsdowntargetlevelid))))